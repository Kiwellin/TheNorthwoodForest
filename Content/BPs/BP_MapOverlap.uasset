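; BP_MapOverlap is a trigger that updates the location shown in the player's NoteBook as the player moves through it.
; It caches the first-person character at BeginPlay, and each of its two boxes passes its own map point to NoteBook.UpdateLocation when that character begins overlapping.
; Disconnected debug logic would detect crossing direction from a dot product against Box1's forward vector, but it never runs.
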(event `self.ReceiveBeginPlay`
  (bind _asbp_first_person_character (cast `/Game/BPs/Player/BP_FirstPersonCharacter` (`GameplayStatics.GetPlayerPawn` 0)))
  (set `self.Player` _asbp_first_person_character))

(event `self.Box1.OnComponentEndOverlap`
  (params (OverlappedComponent :type "PrimitiveComponent Object Reference") (OtherActor :type "Actor Object Reference") (OtherComp :type "PrimitiveComponent Object Reference") (OtherBodyIndex :type Integer)))

(event `self.Box1.OnComponentBeginOverlap`
  (params (OverlappedComponent :type "PrimitiveComponent Object Reference") (OtherActor :type "Actor Object Reference") (OtherComp :type "PrimitiveComponent Object Reference") (OtherBodyIndex :type Integer) (bFromSweep :type Boolean) (SweepResult :type "HitResult Structure (by ref)"))
  (if (== (`self.Player`) OtherActor)
    (`/Game/UI/Notebook/BPW_Notebook.UpdateLocation` (`/Game/BPs/Player/BP_FirstPersonCharacter.NoteBook` (`self.Player`)) (`self.MapPoint1`))))

(event `self.Box2.OnComponentBeginOverlap`
  (params (OverlappedComponent :type "PrimitiveComponent Object Reference") (OtherActor :type "Actor Object Reference") (OtherComp :type "PrimitiveComponent Object Reference") (OtherBodyIndex :type Integer) (bFromSweep :type Boolean) (SweepResult :type "HitResult Structure (by ref)"))
  (if (== (`self.Player`) OtherActor)
    (`/Game/UI/Notebook/BPW_Notebook.UpdateLocation` (`/Game/BPs/Player/BP_FirstPersonCharacter.NoteBook` (`self.Player`)) (`self.MapPoint2`))))

(fn `UserConstructionScript`)