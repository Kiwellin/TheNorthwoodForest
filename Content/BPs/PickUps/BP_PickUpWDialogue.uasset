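; BP_PickUpWDialogue is a pickup actor that plays dialogue when a player interacts with it.
; Interact requires a valid Dialogue table, then uses CanPickUp to assign either it or NoBridgeYetDialogue to BPItemDialogueComp and starts the interact dialogue.
; Interact always returns false, and the event graph and construction script add no logic of their own.
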(fn `Interact`
  (params (`Player Character` :type "/Game/BPs/Player/BP_FirstPersonCharacter Object Reference") (PickUpItem :type "/Game/BPs/PickUps/BP_PickUpItem Object Reference"))
  (returns (UsedPickUp :type Boolean))
  (`/Engine/EditorBlueprintResources/StandardMacros.IsValid` (`self.Dialogue`)
    (:`Is Valid`
      (if (`self.CanPickUp?`)
        (set `/Game/BPs/BP_ItemDialogueComp.Dialogue Data Table` (`self.Dialogue`) (`self.BP_ItemDialogueComp`))
        (else
          (set `/Game/BPs/BP_ItemDialogueComp.Dialogue Data Table` (`self.NoBridgeYetDialogue`) (`self.BP_ItemDialogueComp`))))
      (`/Game/BPs/BP_ItemDialogueComp.StartInteractDialogue` (`self.BP_ItemDialogueComp`)))
    (:`Is Not Valid`
      _))
  (return false))

(fn `UserConstructionScript`
  (`parent.UserConstructionScript`))