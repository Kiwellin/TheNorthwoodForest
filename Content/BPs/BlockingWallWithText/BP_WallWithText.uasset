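; Blocking wall that shows a random-row dialogue widget when the player enters its overlap box, and disappears once its linked sorting puzzles are solved.
; Each puzzle reports through AddCorrect; when all are solved, looping footstep audio starts ahead of the camera and a timeline pulls it toward the player.
; A looping timer uses a dot product to destroy the wall, puzzle actors and their attachments only while the player looks away.
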(event `self.ReceiveBeginPlay`
  (bind _asbp_first_person_character (cast `/Game/BPs/Player/BP_FirstPersonCharacter` (`GameplayStatics.GetPlayerPawn` 0)))
  (set `self.As BP First Person Character` _asbp_first_person_character)
  (for _array_element (`self.SortingPuzzle`)
    (add `/Game/BPs/PlaceItem/BP_PlaceItemTarget.Item/sSolved` _array_element (delegate `Add Correct`))))

(event `Add Correct`
  (`/Engine/EditorBlueprintResources/StandardMacros.IncrementInt` (`self.CorrectSorted`)
    (:`  `
      (`self.CheckIfAllCorrect`))))

(event `self.OverlapBox.OnComponentBeginOverlap`
  (params (OverlappedComponent :type "PrimitiveComponent Object Reference") (OtherActor :type "Actor Object Reference") (OtherComp :type "PrimitiveComponent Object Reference") (OtherBodyIndex :type Integer) (bFromSweep :type Boolean) (SweepResult :type "HitResult Structure (by ref)"))
  (bind _dialogue_data_table (`self.Dialogue Data Table`))
  (if (== OtherActor (`self.As BP First Person Character`))
    (`/Engine/EditorBlueprintResources/StandardMacros.IsValid` (`self.DialogueWidget`)
      (:`Is Not Valid`
        (bind _returnvalue (`|CreateWidget` "/Game/UI/Dialogue/BPW_Dialogue.BPW_Dialogue_C"))
        (bind _output_get (set `self.DialogueWidget` _returnvalue))
        (set `/Game/UI/Dialogue/BPW_Dialogue.DialogueDataTable` _dialogue_data_table _output_get)
        (bind _outrownames (`DataTableFunctionLibrary.GetDataTableRowNames` _dialogue_data_table))
        (set `/Game/UI/Dialogue/BPW_Dialogue.RowNumber` (+ (`.OutIndex` (`KismetArrayLibrary.Array_Random` _outrownames)) 1) (`self.DialogueWidget`))
        (`UserWidget.AddToViewport` (`self.DialogueWidget`) 0)
        (add `/Game/UI/Dialogue/BPW_Dialogue.CallEnded` (`self.DialogueWidget`) (delegate `RemoveWidget`))))))

(event `RemoveWidget`
  (`Widget.RemoveFromParent` (`self.DialogueWidget`))
  (set `self.DialogueWidget` null))

(event `PuzzleSolved`
  (bind _camera (`/Game/BPs/Player/BP_FirstPersonCharacter.Camera` (`self.As BP First Person Character`)))
  (bind _returnvalue (- (`SceneComponent.K2_GetComponentLocation` _camera) (* (`SceneComponent.GetForwardVector` _camera) -2000.0)))
  (`SceneComponent.K2_SetWorldLocation` (`self.SC_Footsteps`) _returnvalue false false)
  (set `self.StartVectSound` _returnvalue)
  (`KismetSystemLibrary.K2_SetTimer` null "CheckIfPlayer is looking away" 0.1 true)
  (bind _returnvalue_2 (`KismetSystemLibrary.K2_SetTimer` null "LoopFootsteps" 0.22 true))
  (bind (_direction _timeline) (`Timeline|FeetCloser` :!via `PlayFromStart`)
    (:`Update`
      (`SceneComponent.K2_SetWorldLocation` (`self.SC_Footsteps`) (`KismetMathLibrary.VLerp` (`self.StartVectSound`) (`SceneComponent.K2_GetComponentLocation` (`/Game/BPs/Player/BP_FirstPersonCharacter.Camera` (`self.As BP First Person Character`))) _timeline) false false))
    (:`Finished`
      (`KismetSystemLibrary.K2_ClearAndInvalidateTimerHandle` _returnvalue_2))))

(fn `CheckIfAllCorrect`
  (if (== (`KismetArrayLibrary.Array_Length` (`self.SortingPuzzle`)) (`self.CorrectSorted`))
    (`self.PuzzleSolved`)))

(fn `CheckIfPlayer is looking away`
  (if (> (* (`KismetMathLibrary.Dot_VectorVector` (`KismetMathLibrary.GetForwardVector` (`KismetMathLibrary.FindLookAtRotation` (`self.K2_GetActorLocation`) (`self.K2_GetActorLocation` (`self.As BP First Person Character`)))) (`SceneComponent.GetForwardVector` (`/Game/BPs/Player/BP_FirstPersonCharacter.Camera` (`self.As BP First Person Character`)))) 1.0) 0.5)
    (for _array_element (`self.SortingPuzzle`)
      (for _array_element_2 (`self.GetAttachedActors` _array_element true false)
        (`self.K2_DestroyActor` _array_element_2))
      (`self.K2_DestroyActor` _array_element))
    (`self.K2_DestroyActor`)
    (else
      (`KismetSystemLibrary.PrintString` "ffffHello"))))

(fn `LoopFootsteps`
  (bind _sc_footsteps (`self.SC_Footsteps`))
  (`AudioComponent.Play` _sc_footsteps 0.0)
  (`KismetSystemLibrary.PrintString` (`KismetStringLibrary.Conv_VectorToString` (`SceneComponent.K2_GetComponentLocation` _sc_footsteps))))

(fn `UserConstructionScript`)