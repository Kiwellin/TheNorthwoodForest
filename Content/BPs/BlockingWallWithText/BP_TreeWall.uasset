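; Tree wall Blueprint that removes itself, unseen by the player, once its linked Flashlight puzzle is solved.
; On solve, a timeline moves a footstep sound from Start to End while a looping timer replays it.
; Another timer compares the wall-to-player direction with camera forward by dot product, destroying the wall when the player faces almost directly away.
; Debug prints remain, and CheckIfAllCorrect is never called here.
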(event `self.ReceiveBeginPlay`
  (bind _asbp_first_person_character (cast `/Game/BPs/Player/BP_FirstPersonCharacter` (`GameplayStatics.GetPlayerPawn` 0)))
  (set `self.As BP First Person Character` _asbp_first_person_character)
  (add `/Game/BPs/Flashlight/BP_FlashlightPuzzle.Solved` (`self.Flashlight`) (delegate `PuzzleSolved`)))

(event `PuzzleSolved`
  (`KismetSystemLibrary.K2_SetTimer` null "CheckIfPlayer is looking away" 0.1 true)
  (bind _returnvalue (`KismetSystemLibrary.K2_SetTimer` null "LoopFootsteps" 0.22 true))
  (bind (_direction _timeline) (`Timeline|FeetCloser` :!via `PlayFromStart`)
    (:`Update`
      (`SceneComponent.K2_SetWorldLocation` (`self.SC_Footsteps`) (`KismetMathLibrary.VLerp` (`SceneComponent.K2_GetComponentLocation` (`self.start`)) (`SceneComponent.K2_GetComponentLocation` (`self.end`)) _timeline) false false))
    (:`Finished`
      (`KismetSystemLibrary.K2_ClearAndInvalidateTimerHandle` _returnvalue))))

(fn `CheckIfAllCorrect`
  (returns (AllCorrect :type Boolean))
  (for _array_element _
    (if (== _array_element false)
      (return false)))
  (return true))

(fn `CheckIfPlayer is looking away`
  (bind _returnvalue (* (`KismetMathLibrary.Dot_VectorVector` (`KismetMathLibrary.GetForwardVector` (`KismetMathLibrary.FindLookAtRotation` (`self.K2_GetActorLocation`) (`self.K2_GetActorLocation` (`self.As BP First Person Character`)))) (`SceneComponent.GetForwardVector` (`/Game/BPs/Player/BP_FirstPersonCharacter.Camera` (`self.As BP First Person Character`)))) 1.0))
  (`KismetSystemLibrary.PrintString` (`KismetStringLibrary.Conv_DoubleToString` _returnvalue))
  (if (> _returnvalue 0.9)
    (`self.K2_DestroyActor`)
    (else
      (`KismetSystemLibrary.PrintString` "ffffHello"))))

(fn `LoopFootsteps`
  (bind _sc_footsteps (`self.SC_Footsteps`))
  (`AudioComponent.Play` _sc_footsteps 0.0)
  (`KismetSystemLibrary.PrintString` (`KismetStringLibrary.Conv_VectorToString` (`SceneComponent.K2_GetComponentLocation` _sc_footsteps))))

(fn `UserConstructionScript`)