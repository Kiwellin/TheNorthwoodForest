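; BP_RepairORMultiPlace is a placement Blueprint that takes several required items, as for a repair or multi-item spot.
; On CheckPlacedItem it removes the placed item from NeededItems, destroys that actor and re-enables its own collision.
; An empty list calls ItemIsCorrect; otherwise ItemsNotYetCorrect fires, an event left empty here.
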(event `self.CheckPlacedItem`
  (params (Player :type "/Game/BPs/Player/BP_FirstPersonCharacter Object Reference"))
  (bind _neededitems (`self.NeededItems`))
  (`KismetArrayLibrary.Array_RemoveItem` _neededitems (`|GetArrayItem` _neededitems (`KismetArrayLibrary.Array_Find` _neededitems (`self.PlacedItem`))))
  (`self.K2_DestroyActor` (`self.PlacedItem`))
  (set `self.PlacedItem` null)
  (`self.SetActorEnableCollision` true)
  (if (== (`KismetArrayLibrary.Array_Length` (`self.NeededItems`)) 0)
    (`self.ItemIsCorrect`)
    (else
      (`self.ItemsNotYetCorrect`))))

(event `ItemsNotYetCorrect`)

(fn `UserConstructionScript`
  (`parent.UserConstructionScript`))