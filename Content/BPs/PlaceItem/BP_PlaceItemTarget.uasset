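; BP_PlaceItemTarget is an interactable spot where the player places a carried item, checked against a designated CorrectItem.
; Interact accepts an item only while PlaceTarget has no child, then PlaceItem reparents it there and re-enables its mesh collision.
; CheckPlacedItem marks a match as correct, fires ItemsSolved and disables the item's collision.
; CanPickUpItemAgain currently has no effect, and debug prints remain.
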(event `CheckPlacedItem`
  (params (Player :type "/Game/BPs/Player/BP_FirstPersonCharacter Object Reference") (Item :type "/Game/BPs/PickUps/BP_PickUpItem Object Reference"))
  (bind _placeditem (`self.PlacedItem`))
  (bind _correctitem (`self.CorrectItem`))
  (`KismetSystemLibrary.PrintString` (`KismetSystemLibrary.GetDisplayName` _placeditem))
  (`KismetSystemLibrary.PrintString` (`KismetSystemLibrary.GetDisplayName` _correctitem))
  (if (== _placeditem _correctitem)
    (`self.ItemIsCorrect`)
    (set `self.ItemCorrect` true)))

(event `ItemIsCorrect`
  (`self.Item/sSolved`)
  (`self.SetActorEnableCollision` (`self.PlacedItem`) false))

(fn `Interact`
  (params (`Player Character` :type "/Game/BPs/Player/BP_FirstPersonCharacter Object Reference") (PickUpItem :type "/Game/BPs/PickUps/BP_PickUpItem Object Reference"))
  (returns (UsedPickUp :type Boolean))
  (`/Engine/EditorBlueprintResources/StandardMacros.IsValid` (`SceneComponent.GetChildComponent` (`self.PlaceTarget`) 0)
    (:`Is Not Valid`
      (`/Engine/EditorBlueprintResources/StandardMacros.IsValid` PickUpItem
        (:`Is Valid`
          (`KismetSystemLibrary.PrintString` "Hello")
          (`self.PlaceItem` PickUpItem)
          (`self.CheckPlacedItem` `Player Character`)
          (return true))
        (:`Is Not Valid`
          (`KismetSystemLibrary.PrintString` "dddd"))))))

(fn `PlaceItem`
  (params (PlaceItem :type "/Game/BPs/PickUps/BP_PickUpItem Object Reference"))
  (bind _output_get (set `self.PlacedItem` PlaceItem))
  (`/Game/BPs/PickUps/BP_PickUpItem.ChangeParents` _output_get (`self.PlaceTarget`))
  (`PrimitiveComponent.SetCollisionEnabled` (`/Game/BPs/PickUps/BP_PickUpItem.StaticMesh` _output_get) "QueryAndPhysics")
  (if (`self.CanPickUpItemAgain`)
    _))

(fn `UserConstructionScript`)