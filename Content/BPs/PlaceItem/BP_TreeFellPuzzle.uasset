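; Item-placement puzzle actor where the correct item fells a tree.
; A correct item plays the falling level sequence at reduced speed; a failed parent Interact starts item dialogue instead.
; A separate TreeFallin event reveals the fallen log, swaps the mesh, destroys the placed item and runs a timeline.
; The timeline rolls the mesh to its target rotation, then removes the box component.
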(event `self.ReceiveBeginPlay`
  (set `self.StartRot` (`SceneComponent.RelativeRotation` (`self.StaticMesh`))))

(event `self.ItemIsCorrect`
  (bind _sequenceplayer (`LevelSequenceActor.SequencePlayer` (`self.LS-Falling`)))
  (`MovieSceneSequencePlayer.SetPlayRate` _sequenceplayer 0.6)
  (`MovieSceneSequencePlayer.Play` _sequenceplayer))

(event `TreeFallin`
  (bind (_startrot_roll _startrot_pitch _startrot_yaw) (`KismetMathLibrary.BreakRotator` (`self.StartRot`)))
  (`SceneComponent.SetHiddenInGame` (`self.fallenlog`) false false)
  (`StaticMeshComponent.SetStaticMesh` (`self.StaticMesh`) (`self.ChangedMesh`))
  (`self.K2_DestroyActor` (`self.PlacedItem`))
  (bind (_direction _fall) (`Timeline|fallin tree`)
    (:`Update`
      (`SceneComponent.K2_SetRelativeRotation` (`self.StaticMesh`) (`KismetMathLibrary.MakeRotator` (`KismetMathLibrary.Lerp` 90.0 (`self.TargetRot`) _fall) _startrot_pitch _startrot_yaw) false false))
    (:`Finished`
      (`ActorComponent.K2_DestroyComponent` (`self.Box`)))))

(fn `Interact`
  (params (`Player Character` :type "/Game/BPs/Player/BP_FirstPersonCharacter Object Reference") (PickUpItem :type "/Game/BPs/PickUps/BP_PickUpItem Object Reference"))
  (returns (UsedPickUp :type Boolean))
  (bind _usedpickup (`parent.Interact` `Player Character` PickUpItem))
  (if _usedpickup
    (return _usedpickup)
    (else
      (`/Game/BPs/BP_ItemDialogueComp.StartInteractDialogue` (`self.BP_ItemDialogueComp`))
      (return false))))

(fn `UserConstructionScript`
  (`parent.UserConstructionScript`))