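; BP_Cable is a cable actor that tracks which ports it is plugged into, apparently for a cable-connection puzzle.
; It disables its collision on BeginPlay, and AttachedToPort stores each port in a map keyed by cable part.
; CheckForRemovedCorrectPorts counts attached ports with a correct cable, clears the map and returns that count with a removal flag.
; The two-port check and CheckCorrectCable loop are unfinished or unwired.
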(event `self.ReceiveBeginPlay`
  (`self.SetActorEnableCollision` false))

(event `AttachedToPort`
  (params (Port :type "/Game/BPs/CableConnect/BP_ConnectPort Object Reference") (CablePart :type "StaticMeshComponent Object Reference"))
  (`BlueprintMapLibrary.Map_Add` (`self.AttachedPorts`) CablePart Port)
  (if (>= (`BlueprintMapLibrary.Map_Length` (`self.AttachedPorts`)) 2)
    _))

(fn `CheckForRemovedCorrectPorts`
  (returns (`RemovedFromPorts?` :type Boolean) (AmountRemoved :type Integer))
  (locals (Amount :type Integer))
  (bind _attachedports (`self.AttachedPorts`))
  (if (> (`BlueprintMapLibrary.Map_Length` (`self.AttachedPorts`)) 0)
    (`KismetSystemLibrary.PrintString` "remove")
    (set `local.Amount` 0)
    (bind (_keypin _valuepin) (`|MapForEach` _attachedports)
      (:`then`
        (if (`/Game/BPs/CableConnect/BP_ConnectPort.HasCorrectCable` _valuepin)
          (`/Engine/EditorBlueprintResources/StandardMacros.IncrementInt` (`local.Amount`))))
      (:`CompletedPin`
        (`BlueprintMapLibrary.Map_Clear` _attachedports)
        (return true (`local.Amount`))))
    (else
      (`KismetSystemLibrary.PrintString` "nothing to remove")
      (return false 0))))

(fn `UserConstructionScript`)