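; BP_ConnectPort is a port for cable connections that tracks which cable occupies it and whether that cable is the correct one.
; CheckCorrectCable stores the passed cable, compares it to CorrectCable, then saves and returns the result as HasCorrectCable.
; CheckCableStatus returns true when the port holds no valid cable.
; ResetCableStatus clears the stored cable and prints a debug message, leaving HasCorrectCable unchanged.
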(event `ResetCableStatus`
  (set `self.Cable` null)
  (`KismetSystemLibrary.PrintString` "cable reset"))

(fn `CheckCableStatus`
  (returns (NoCableConnected :type Boolean))
  (`/Engine/EditorBlueprintResources/StandardMacros.IsValid` (`self.Cable`)
    (:`Is Valid`
      (return false))
    (:`Is Not Valid`
      (return true))))

(fn `CheckCorrectCable`
  (params (Cable :type "/Game/BPs/CableConnect/BP_Cable Object Reference"))
  (returns (WasRightCable :type Boolean))
  (set `self.Cable` Cable)
  (if (== (`self.Cable`) (`self.CorrectCable`))
    (bind _output_get (set `self.HasCorrectCable` true))
    (return _output_get)
    (else
      (bind _output_get_2 (set `self.HasCorrectCable` false))
      (return _output_get_2))))