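; Flashlight puzzle actor that blinks a looping short/long light pattern for the player to copy with their flashlight.
; A self-recalling PlayLight event times the spotlight from the Lights array, pausing longer when it wraps.
; Player flick dispatchers record short or long flashes, and the player's timer expiry clears them.
; An exact array match removes the player's flashlight, broadcasts Solved and destroys the actor.
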(event `self.ReceiveBeginPlay`
  (`self.PlayLight`)
  (bind _asbp_first_person_character (cast `/Game/BPs/Player/BP_FirstPersonCharacter` (`GameplayStatics.GetPlayerPawn` 0)))
  (set `self.Player` _asbp_first_person_character)
  (add `/Game/BPs/Player/BP_FirstPersonCharacter.CallLightFlicked` (`self.Player`) (delegate `ShortLight_Event`))
  (add `/Game/BPs/Player/BP_FirstPersonCharacter.CallTimerRunOut` (`self.Player`) (delegate `CallTimerRunOut_Event`)))

(event `CallTimerRunOut_Event`
  (`KismetArrayLibrary.Array_Clear` (`self.PlayerLightArray`))
  (`KismetSystemLibrary.PrintString` "cleared"))

(event `ShortLight_Event`
  (params (`Was Short?` :type Boolean))
  (if `Was Short?`
    (`KismetArrayLibrary.Array_Add` (`self.PlayerLightArray`) 0.5)
    (else
      (`KismetArrayLibrary.Array_Add` (`self.PlayerLightArray`) 1.5)))
  (bind _correctcode (`self.CheckCode`))
  (if _correctcode
    (`KismetSystemLibrary.PrintString` "correct")
    (set `/Game/BPs/Player/BP_FirstPersonCharacter.HasFlashlight` false (`self.Player`))
    (`self.Solved`)
    (`self.K2_DestroyActor`)
    (else
      (`KismetSystemLibrary.PrintString` "WROOOONG"))))

(event `PlayLight`
  (bind _lightindex (`self.LightIndex`))
  (`SceneComponent.SetHiddenInGame` (`self.SpotLight`) true true)
  (`KismetSystemLibrary.Delay` (`self.ResetTime`))
  (`SceneComponent.SetHiddenInGame` (`self.SpotLight`) false true)
  (`/Engine/EditorBlueprintResources/StandardMacros.IncrementInt` _lightindex
    (:`  `
      (`self.Clamp`)
      (bind _output_get (set `self.Time` (`|GetArrayItem` (`self.Lights`) _lightindex)))
      (`KismetSystemLibrary.Delay` _output_get)
      (`self.PlayLight`))))

(fn `CheckCode`
  (returns (CorrectCode :type Boolean))
  (if (== (`KismetArrayLibrary.Array_Length` (`self.Lights`)) (`KismetArrayLibrary.Array_Length` (`self.PlayerLightArray`)))
    (return (`KismetArrayLibrary.Array_Identical` (`self.PlayerLightArray`) (`self.Lights`)))))

(fn `Clamp`
  (`|ExecutionSequence`
    (:`then_0`
      (if (< (`self.LightIndex`) (`KismetArrayLibrary.Array_Length` (`self.Lights`)))
        (set `self.ResetTime` 0.2)))
    (:`then_1`
      (if (>= (`self.LightIndex`) (`KismetArrayLibrary.Array_Length` (`self.Lights`)))
        (set `self.LightIndex` 0)
        (set `self.ResetTime` 2.0)))))

(fn `UserConstructionScript`)