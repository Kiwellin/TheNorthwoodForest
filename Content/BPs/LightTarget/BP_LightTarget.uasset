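; Light puzzle target that is solved when the required number of spyglasses hit it at once.
; On BeginPlay it binds to each spyglass's hit event, adding or removing that spyglass from a unique list of correct hits.
; The normalized hit count drives Niagara smoke.
; When solved, it pauses the spyglasses' LightStart timers, activates a particle effect and makes them no longer possessable.
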(event `self.ReceiveBeginPlay`
  (for _array_element (`self.Spyglasses`)
    (add `/Game/BPs/Interactables/SpyglassPuzzle/BP_Spyglass.HitSomething` _array_element (delegate `HitSomething`))))

(event `HitSomething`
  (params (HitActor :type "Actor Object Reference") (Spyglass :type "/Game/BPs/Interactables/SpyglassPuzzle/BP_Spyglass Object Reference"))
  (`self.Check If LightWasHit` HitActor Spyglass)
  (bind _all_done (`self.CheckLights`))
  (`NiagaraComponent.SetVariableFloat` (`self.Niagara`) "SmokeAmount" (`KismetMathLibrary.NormalizeToRange` (`KismetMathLibrary.Conv_IntToDouble` (`KismetArrayLibrary.Array_Length` (`self.CorrectHitSpyglasses`))) 0.0 (`KismetMathLibrary.Conv_IntToDouble` (`self.Amount of Light Needed`))))
  (if _all_done
    (`self.Solved`)))

(event `Solved`
  (for _array_element (`self.Spyglasses`)
    (`KismetSystemLibrary.K2_PauseTimer` _array_element "LightStart"))
  (`ActorComponent.Activate` (`self.ParticleSystem`) false)
  (for _array_element_2 (`self.Spyglasses`)
    (set `/Game/BPs/InteractablePossessables/BP_InteractablePossessable.CanBePossessed?` false _array_element_2)))

(fn `Check If LightWasHit`
  (params (HitActor :type "Object Object Reference") (SpyglassActor :type "/Game/BPs/Interactables/SpyglassPuzzle/BP_Spyglass Object Reference (by ref)"))
  (returns (Spyglass :type "/Game/BPs/Interactables/SpyglassPuzzle/BP_Spyglass Object Reference"))
  (locals (SpyglassAct :type "/Game/BPs/Interactables/SpyglassPuzzle/BP_Spyglass Object Reference"))
  (set `local.SpyglassAct` SpyglassActor)
  (if (== HitActor self)
    (`KismetArrayLibrary.Array_AddUnique` (`self.CorrectHitSpyglasses`) (`local.SpyglassAct`))
    (return (`local.SpyglassAct`))
    (else
      (`KismetArrayLibrary.Array_RemoveItem` (`self.CorrectHitSpyglasses`) (`local.SpyglassAct`))
      (return (`local.SpyglassAct`)))))

(fn `CheckLights`
  (returns (`All Done` :type Boolean))
  (return (== (`self.Amount of Light Needed`) (`KismetArrayLibrary.Array_Length` (`self.CorrectHitSpyglasses`)))))

(fn `UserConstructionScript`)