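; BP_StonesFallingCollission is a one-shot trigger that sends stones falling when the first-person character enters its Box.
; On overlap it plays audio, destroys the Box, then enables physics and applies impulses to referenced Geometry Collection and static mesh stones.
; The Cube's collision is disabled at BeginPlay and switches to query and physics once the fall is triggered.
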(event `self.ReceiveBeginPlay`
  (`PrimitiveComponent.SetCollisionEnabled` (`self.Cube`) "NoCollision"))

(event `self.Box.OnComponentBeginOverlap`
  (params (OverlappedComponent :type "PrimitiveComponent Object Reference") (OtherActor :type "Actor Object Reference") (OtherComp :type "PrimitiveComponent Object Reference") (OtherBodyIndex :type Integer) (bFromSweep :type Boolean) (SweepResult :type "HitResult Structure (by ref)"))
  (cast `/Game/BPs/Player/BP_FirstPersonCharacter` OtherActor)
  (`AudioComponent.Play` (`self.Audio`) 0.0)
  (`ActorComponent.K2_DestroyComponent` (`self.Box`))
  (`self.FallStones`)
  (`PrimitiveComponent.SetCollisionEnabled` (`self.Cube`) "QueryAndPhysics"))

(event `FallStones`
  (for _array_element (`self.GC-FallingStones`)
    (bind _geometrycollectioncomponent (`GeometryCollectionActor.GeometryCollectionComponent` _array_element))
    (`PrimitiveComponent.SetSimulatePhysics` _geometrycollectioncomponent true)
    (`PrimitiveComponent.AddImpulse` _geometrycollectioncomponent (`self.ImpulseGC`) "None" false))
  (for _array_element_2 (`self.SM-Fallingstones`)
    (bind _stone (`/Game/BPs/Stone/BP_SMStone.stone` _array_element_2))
    (`PrimitiveComponent.SetSimulatePhysics` _stone true)
    (`PrimitiveComponent.AddImpulse` _stone (`self.Impulse`) "None" false)))

(fn `UserConstructionScript`)