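; BP_Tent is an interactable tent that lets the player rest to change the time of day.
; Interacting while rest is allowed fades the camera out, disables input, changes daytime through the game mode and notifies CampGate.
; It then clears CanRest, restores input, fires the Slept dispatcher and fades back in.
; When rest is not allowed, it starts the item dialogue component's interact dialogue if a dialogue table is set.
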(event `AttemptTimeChange`
  (bind _bp_itemdialoguecomp (`self.BP_ItemDialogueComp`))
  (if (`self.CanRest?`)
    (`PlayerCameraManager.StartCameraFade` :`self` (`GameplayStatics.GetPlayerCameraManager` 0) :`ToAlpha` 1.0 :`Duration` (`self.CamFadeDuration`) :`bHoldWhenFinished` true)
    (`self.DisableInput` (`GameplayStatics.GetPlayerPawn` 0) (`GameplayStatics.GetPlayerController` 0))
    (`self.DisableInput` (`GameplayStatics.GetPlayerController` 0) (`GameplayStatics.GetPlayerController` 0))
    (`KismetSystemLibrary.Delay` (`self.CamFadeDuration`))
    (bind _gamemode (message `/Game/BPs/BPI/BPI_GameModeRef.GameModeRef` (`GameplayStatics.GetGameMode`)))
    (`/Game/Game_mode-Game_instance/BP_Gamemode.ChangeDaytime` _gamemode)
    (set `self.CanRest?` false)
    (`/Game/BPs/Interactables/Tent/BP_Campgates.Rested` (`self.CampGate`))
    (`KismetSystemLibrary.Delay` (`self.CamFadeDuration`))
    (`self.EnableInput` (`GameplayStatics.GetPlayerPawn` 0) (`GameplayStatics.GetPlayerController` 0))
    (`self.Slept`)
    (`PlayerCameraManager.StartCameraFade` :`self` (`GameplayStatics.GetPlayerCameraManager` 0) :`FromAlpha` 1.0 :`Duration` (`self.CamFadeDuration`))
    (else
      (`/Engine/EditorBlueprintResources/StandardMacros.IsValid` (`/Game/BPs/BP_ItemDialogueComp.Dialogue Data Table` _bp_itemdialoguecomp)
        (:`Is Valid`
          (`/Game/BPs/BP_ItemDialogueComp.StartInteractDialogue` _bp_itemdialoguecomp))))))

(fn `Interact`
  (params (`Player Character` :type "/Game/BPs/Player/BP_FirstPersonCharacter Object Reference") (PickUpItem :type "/Game/BPs/PickUps/BP_PickUpItem Object Reference"))
  (returns (UsedPickUp :type Boolean))
  (`self.AttemptTimeChange`)
  (return false))

(fn `UserConstructionScript`)