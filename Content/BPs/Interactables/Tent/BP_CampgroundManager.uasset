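; BP_CampgroundManager coordinates a set of campground gates and an optional level sequence with dialogue.
; It binds to each gate's dispatchers, relaying passage state and the dialogue widget to all gates.
; When a gate reports the player positioned, it plays the sequence, toggles the HUD, shows dialogue and disables input.
; When the dialogue call ends, it removes the widget, stops the sequence and restores input and camera with a fade.
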(event `self.ReceiveBeginPlay`
  (for _array_element (`self.Gates`)
    (add `/Game/BPs/Interactables/Tent/BP_Campgates.PassageDe/Activation` _array_element (delegate `PassageDe/Activate`))
    (add `/Game/BPs/Interactables/Tent/BP_Campgates.DialogueWidgetCall` _array_element (delegate `SetDialogueForAll`))
    (add `/Game/BPs/Interactables/Tent/BP_Campgates.PlayerPositionSet` _array_element (delegate `CheckForLS`))))

(event `PassageDe/Activate`
  (params (`CanPass?` :type Boolean))
  (for _array_element (`self.Gates`)
    (`/Game/BPs/Interactables/Tent/BP_Campgates.PassageDe/Activate` _array_element `CanPass?`)))

(event `SetDialogueForAll`
  (params (DialogueWidget :type "/Game/UI/Dialogue/BPW_Dialogue Object Reference"))
  (for _array_element (`self.Gates`)
    (set `/Game/BPs/Interactables/Tent/BP_Campgates.DialogueWidget` DialogueWidget _array_element)))

(event `CheckForLS`
  (`/Engine/EditorBlueprintResources/StandardMacros.IsValid` (`self.LS`)
    (:`Is Valid`
      (`MovieSceneSequencePlayer.Play` (`LevelSequenceActor.SequencePlayer` (`self.LS`)))
      (`self.Level SequenceStart`)
      (add `/Game/UI/Dialogue/BPW_Dialogue.CallEnded` (`self.DialogueWidget`) (delegate `Remove Widget`))
      (`self.DisableInput` (`GameplayStatics.GetPlayerPawn` 0) (`GameplayStatics.GetPlayerController` 0)))))

(event `Remove Widget`
  (`Widget.RemoveFromParent` (`self.DialogueWidget`))
  (set `self.DialogueWidget` null)
  (`MovieSceneSequencePlayer.Stop` (`LevelSequenceActor.SequencePlayer` (`self.LS`)))
  (bind _asbp_first_person_character (cast `/Game/BPs/Player/BP_FirstPersonCharacter` (`GameplayStatics.GetPlayerCharacter` 0)))
  (`/Game/UI/Player/BPW_PlayerHUD.Un/hide HUD` (`/Game/BPs/Player/BP_FirstPersonCharacter.PlayerHUD` _asbp_first_person_character) false)
  (`self.EnableInput` (`GameplayStatics.GetPlayerPawn` 0) (`GameplayStatics.GetPlayerController` 0))
  (bind _asbp_first_person_character_2 (cast `/Game/BPs/Player/BP_FirstPersonCharacter` (`GameplayStatics.GetPlayerCharacter` 0)))
  (`ActorComponent.Activate` (`/Game/BPs/Player/BP_FirstPersonCharacter.Camera` _asbp_first_person_character_2) false)
  (`PlayerCameraManager.StartCameraFade` :`self` (`GameplayStatics.GetPlayerCameraManager` 0) :`FromAlpha` 1.0 :`Duration` 1.0))

(fn `Level SequenceStart`
  (bind _asbp_first_person_character (cast `/Game/BPs/Player/BP_FirstPersonCharacter` (`GameplayStatics.GetPlayerCharacter` 0)))
  (`/Game/UI/Player/BPW_PlayerHUD.Un/hide HUD` (`/Game/BPs/Player/BP_FirstPersonCharacter.PlayerHUD` _asbp_first_person_character) true)
  (`/Engine/EditorBlueprintResources/StandardMacros.IsValid` (`self.DialogueWidget`)
    (:`Is Not Valid`
      (bind _returnvalue (`|CreateWidget` "/Game/UI/Dialogue/BPW_Dialogue.BPW_Dialogue_C"))
      (bind _output_get (set `self.DialogueWidget` _returnvalue))
      (set `/Game/UI/Dialogue/BPW_Dialogue.DialogueDataTable` (`self.Dialogue Data Table`) _output_get)
      (`UserWidget.AddToViewport` (`self.DialogueWidget`) 0)
      (return))))

(fn `UserConstructionScript`)