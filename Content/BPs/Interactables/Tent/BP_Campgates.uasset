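; Camp gate trigger, set as entrance or exit, that controls the player's passage through a camp.
; An open entrance fades the camera, moves the player to its Scene point, then blocks itself and signals PassageDeActivation(false).
; Rested signals true; PassageDeActivate toggles blocking collision on non-entrance gates.
; Blocked attempts open data-table dialogue, random for going back or "rest first" for leaving, with player input disabled until it ends.
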(event `self.ReceiveBeginPlay`)

(event `self.Box.OnComponentBeginOverlap`
  (params (OverlappedComponent :type "PrimitiveComponent Object Reference") (OtherActor :type "Actor Object Reference") (OtherComp :type "PrimitiveComponent Object Reference") (OtherBodyIndex :type Integer) (bFromSweep :type Boolean) (SweepResult :type "HitResult Structure (by ref)"))
  (bind _asbp_first_person_character (cast `/Game/BPs/Player/BP_FirstPersonCharacter` OtherActor))
  (set `self.Player` _asbp_first_person_character)
  (if (`self.IsEntrance?`)
    (if (`self.CanPassEntrance`)
      (`self.NextCampActive`)
      (`self.PassageDe/Activation` false)
      (else
        (`self.CantGoBack`)))
    (else
      (`self.AttemptingToLeaveCamp`))))

(event `CreateDialogue`
  (params (RowNumber :type Integer))
  (`/Engine/EditorBlueprintResources/StandardMacros.IsValid` (`self.DialogueWidget`)
    (:`Is Not Valid`
      (bind _returnvalue (`|CreateWidget` "/Game/UI/Dialogue/BPW_Dialogue.BPW_Dialogue_C"))
      (bind _output_get (set `self.DialogueWidget` _returnvalue))
      (`self.DialogueWidgetCall` _output_get)
      (set `/Game/UI/Dialogue/BPW_Dialogue.DialogueDataTable` (`self.Dialogue Data Table`) _output_get)
      (set `/Game/UI/Dialogue/BPW_Dialogue.RowNumber` RowNumber _output_get)
      (`UserWidget.AddToViewport` (`self.DialogueWidget`) 0)
      (add `/Game/UI/Dialogue/BPW_Dialogue.CallEnded` (`self.DialogueWidget`) (delegate `RemoveWidget`))
      (`self.DisableInput` (`GameplayStatics.GetPlayerCharacter` 0) (`GameplayStatics.GetPlayerController` 0)))))

(event `RemoveWidget`
  (`Widget.RemoveFromParent` (`self.DialogueWidget`))
  (bind _output_get (set `self.DialogueWidget` null))
  (`self.DialogueWidgetCall` _output_get)
  (`self.EnableInput` (`GameplayStatics.GetPlayerCharacter` 0) (`GameplayStatics.GetPlayerController` 0)))

(event `NextCampActive`
  (set `self.CanPassEntrance` false)
  (set `self.CanPass` false)
  (`self.SetPlayerPosition`)
  (`PrimitiveComponent.SetCollisionEnabled` (`self.BlockCol`) "QueryAndPhysics"))

(event `AttemptingToLeaveCamp`
  (if (not (`self.CanPass`))
    (`self.HaveToRestFirst`)))

(event `SetPlayerPosition`
  (`PlayerCameraManager.StartCameraFade` :`self` (`GameplayStatics.GetPlayerCameraManager` 0) :`ToAlpha` 1.0 :`Duration` (`self.CamFadeDuration`) :`bHoldWhenFinished` true)
  (`self.DisableInput` (`self.Player`) (`GameplayStatics.GetPlayerController` 0))
  (`KismetSystemLibrary.Delay` (`self.CamFadeDuration`))
  (`self.K2_SetActorLocation` (`self.Player`) (`SceneComponent.K2_GetComponentLocation` (`self.Scene`)) false false)
  (`KismetSystemLibrary.Delay` (`self.CamFadeDuration`))
  (`self.EnableInput` (`self.Player`) (`GameplayStatics.GetPlayerController` 0))
  (`PlayerCameraManager.StartCameraFade` :`self` (`GameplayStatics.GetPlayerCameraManager` 0) :`FromAlpha` 1.0 :`Duration` (`self.CamFadeDuration`)))

(event `CantGoBack`
  ; pop up
  (bind _output_get (set `self.Dialogue Data Table` (`self.CantGoBackDT`)))
  (bind _outrownames (`DataTableFunctionLibrary.GetDataTableRowNames` _output_get))
  (`self.CreateDialogue` (`KismetStringLibrary.Conv_StringToInt` (`KismetStringLibrary.Conv_NameToString` (`KismetArrayLibrary.Array_Random` _outrownames)))))

(event `HaveToRestFirst`
  ; rest/call first
  (set `self.Dialogue Data Table` (`self.HaveToRest/CallDT`))
  (`self.CreateDialogue` 1))

(event `Rested`
  (`self.PassageDe/Activation` true))

(fn `PassageDe/Activate`
  (params (`CanPass?` :type Boolean))
  (if (not (`self.IsEntrance?`))
    (bind _output_get (set `self.CanPass` `CanPass?`))
    (`PrimitiveComponent.SetCollisionEnabled` (`self.BlockCol`) (select `bool` _output_get :`false` "QueryAndPhysics" :`true` "NoCollision" :!type "ECollisionEnabled Enum"))))

(fn `UserConstructionScript`)