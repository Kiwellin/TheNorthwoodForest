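; Possessable spyglass for a light-beam puzzle, which the player rotates within clamped yaw and roll limits and can exit back to the character.
; A looping timer makes source spyglasses line trace forward, sizing the Niagara beam to the hit distance.
; Spyglasses hit on either box component fire a hit event and, if able to redirect, trace onward recursively, with a game-time check blocking same-frame repeats.
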(event `self.ReceiveTick`
  (params (DeltaSeconds :type "Float (single-precision)"))
  (`parent.ReceiveTick` DeltaSeconds))

(event `self.ReceiveBeginPlay`
  (`parent.ReceiveBeginPlay`)
  (`self.SetVFXEnabled` (`self.IsSource?`))
  (`KismetSystemLibrary.DelayUntilNextTick`)
  (`KismetSystemLibrary.K2_SetTimerDelegate` (delegate `LightStart`) 0.2 true)
  (`KismetArrayLibrary.Array_AddUnique` (`self.Actors to Ignore`) (`self.Player Character`))
  (for _array_element (`self.Actors to Ignore`)
    (`KismetSystemLibrary.PrintString` (`KismetSystemLibrary.GetDisplayName` _array_element))))

(event `LightStart`
  (if (`self.IsSource?`)
    (`self.EmmitLight`)
    (elif (`self.TimeHasPassedSinceLastHit`)
      (`self.SetVFXEnabled` false))))

(event `GetHitByLight`
  (params (HitComponent :type "PrimitiveComponent Object Reference"))
  (if (or (== HitComponent (`self.Box`)) (== HitComponent (`self.Box1`)))
    (if (`self.TimeHasPassedSinceLastHit`)
      (set `self.LastHitTime` (`KismetSystemLibrary.GetGameTimeInSeconds`))
      (`self.OnHitByLight`)
      (if (`self.CanRedirectLight`)
        (`self.SetVFXEnabled` true)
        (`self.EmmitLight`)))))

(event `EnhancedInput|/Game/Input/Actions/IA_RotateCamera`
  (params (ActionValue :type "Vector2D Structure") (ElapsedSeconds :type "Float (double-precision)") (TriggeredSeconds :type "Float (double-precision)") (InputAction :type "InputAction Object Reference" :default "/Game/Input/Actions/IA_RotateCamera.IA_RotateCamera"))
  (:`Triggered`
    (`self.AddSpyglassMovement` ActionValue_X ActionValue_Y)
    (`self.SetActorTickEnabled` true)))

(event `self.GetPossessed`
  (`parent.GetPossessed`))

(event `EnhancedInput|/Game/Input/Actions/IA_ExitPuzzle`
  (params (ActionValue :type Boolean) (ElapsedSeconds :type "Float (double-precision)") (TriggeredSeconds :type "Float (double-precision)") (InputAction :type "InputAction Object Reference" :default "/Game/Input/Actions/IA_ExitPuzzle.IA_ExitPuzzle"))
  (:`Triggered`
    (`self.ReturnToCharacter`)
    (if (not (`self.CanBePossessed?`))
      (`self.PlayDia`))))

(event `self.PlaySolved`
  (`parent.PlaySolved`))

(fn `AddSpyglassMovement`
  (params (LeftRight :type "Float (double-precision)") (UpDown :type "Float (double-precision)"))
  (`SceneComponent.K2_AddLocalRotation` (`self.StaticMesh`) (`KismetMathLibrary.MakeRotator` 0.0 0.0 (* LeftRight (`GameplayStatics.GetWorldDeltaSeconds`) (`self.Rotation Speed`))) false false)
  (`self.ClampLeftRightRotation`)
  (`SceneComponent.K2_AddLocalRotation` (`self.StaticMesh1`) (`KismetMathLibrary.MakeRotator` (* (* UpDown (`GameplayStatics.GetWorldDeltaSeconds`) (`self.Rotation Speed`)) -1.0)) false false)
  (`self.Clamp UpDownRotation`))

(fn `CheckForLightHit`
  (returns (DistanceToHit :type "Float (double-precision)") (HitSomething :type Boolean) (Spyglass :type "/Game/BPs/Interactables/SpyglassPuzzle/BP_Spyglass Object Reference") (HitComponent :type "PrimitiveComponent Object Reference"))
  (bind _lightorigin (`self.LightOrigin`))
  (bind _returnvalue (`SceneComponent.K2_GetComponentLocation` _lightorigin))
  (bind (_outhit _returnvalue_2) (`KismetSystemLibrary.LineTraceSingleForObjects` _returnvalue (+ _returnvalue (* (`SceneComponent.GetForwardVector` _lightorigin) (`self.MaxRange`))) (`|MakeArray` "ObjectTypeQuery1" "ObjectTypeQuery2" "ObjectTypeQuery3" "ObjectTypeQuery4" :!type "EObjectTypeQuery Enum") false (`self.Actors to Ignore`)))
  (if _returnvalue_2
    ; only relevant if light on tick and not on timer
    (`self.SetActorTickEnabled` _returnvalue_2)
    (bind (_bblockinghit _binitialoverlap _time _distance _location _impactpoint _normal _impactnormal _physmat _hitactor _hitcomponent) (`GameplayStatics.BreakHitResult` _outhit))
    (`self.HitSomething` _hitactor self)
    (bind _asbp_spyglass (cast `/Game/BPs/Interactables/SpyglassPuzzle/BP_Spyglass` _hitactor)
      (:`then`
        _)
      (:`CastFailed`
        _))
    (return (`KismetMathLibrary.VSize` (- _impactpoint (`SceneComponent.K2_GetComponentLocation` (`self.LightOrigin`)))) _returnvalue_2 _asbp_spyglass _hitcomponent)
    (else
      (return (`self.MaxRange`) false null null))))

(fn `Clamp UpDownRotation`
  (bind _staticmesh1 (`self.StaticMesh1`))
  (bind (_relativerotation_roll _relativerotation_pitch _relativerotation_yaw) (`KismetMathLibrary.BreakRotator` (`SceneComponent.RelativeRotation` _staticmesh1)))
  (`SceneComponent.K2_SetRelativeRotation` _staticmesh1 (`KismetMathLibrary.MakeRotator` (`KismetMathLibrary.ClampAngle` _relativerotation_roll -30.0 30.0) _relativerotation_pitch _relativerotation_yaw) false false))

(fn `ClampLeftRightRotation`
  (bind _staticmesh (`self.StaticMesh`))
  (bind (_relativerotation_roll _relativerotation_pitch _relativerotation_yaw) (`KismetMathLibrary.BreakRotator` (`SceneComponent.RelativeRotation` _staticmesh)))
  (`SceneComponent.K2_SetRelativeRotation` _staticmesh (`KismetMathLibrary.MakeRotator` _relativerotation_roll _relativerotation_pitch (`KismetMathLibrary.ClampAngle` _relativerotation_yaw 0.0 180.0)) false false))

(fn `EmmitLight`
  (bind (_distancetohit _hitsomething _spyglass _hitcomponent) (`self.CheckForLightHit`))
  (if _hitsomething
    (`NiagaraComponent.SetVariableFloat` (`self.Niagara`) "LightLength" _distancetohit)
    (`/Engine/EditorBlueprintResources/StandardMacros.IsValid` _spyglass
      (:`Is Valid`
        (`self.GetHitByLight` _spyglass _hitcomponent)))
    (else
      (`NiagaraComponent.SetVariableFloat` (`self.Niagara`) "LightLength" _distancetohit))))

(fn `SetVFXEnabled`
  (params (isEnabled :type Boolean))
  (bind _niagara (`self.Niagara`))
  (if isEnabled
    (`ActorComponent.Activate` _niagara false)
    (else
      (`ActorComponent.Deactivate` _niagara))))

(fn `TimeHasPassedSinceLastHit`
  (returns (`Return Value` :type Boolean))
  (return (> (`KismetSystemLibrary.GetGameTimeInSeconds`) (`self.LastHitTime`))))

(fn `UserConstructionScript`
  (`parent.UserConstructionScript`))