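; BP_Readables is an interactable readable that creates a reading widget when the player interacts with it.
; Interact caches the player's HUD, calls UnhideHUD and runs Read, which swaps the character Enhanced Input mapping context for its own and creates the widget; no AddToViewport call happens here.
; The IA_ExitPuzzle action removes the widget, toggles the HUD back and restores the character mapping context.
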(event `Read`
  (`EnhancedInputSubsystemInterface.RemoveMappingContext` (pcsubsystem `EnhancedInputLocalPlayerSubsystem` (`GameplayStatics.GetPlayerController` 0)) (`self.Character Mapping Context`) (struct))
  (`EnhancedInputSubsystemInterface.AddMappingContext` (pcsubsystem `EnhancedInputLocalPlayerSubsystem` (`GameplayStatics.GetPlayerController` 0)) (`self.Mapping Context`) 2 (struct))
  (bind _returnvalue (`|CreateWidget` (`self.ReadWidgetClass`)))
  (set `self.ReadWidget` _returnvalue))

(event `EnhancedInput|/Game/Input/Actions/IA_ExitPuzzle`
  (params (ActionValue :type Boolean) (ElapsedSeconds :type "Float (double-precision)") (TriggeredSeconds :type "Float (double-precision)") (InputAction :type "InputAction Object Reference" :default "/Game/Input/Actions/IA_ExitPuzzle.IA_ExitPuzzle"))
  (:`Triggered`
    (`Widget.RemoveFromParent` (`self.ReadWidget`))
    (`/Game/UI/Player/BPW_PlayerHUD.Un/hide HUD` (`self.Player HUD`) false)
    (`EnhancedInputSubsystemInterface.RemoveMappingContext` (pcsubsystem `EnhancedInputLocalPlayerSubsystem` (`GameplayStatics.GetPlayerController` 0)) (`self.Mapping Context`) (struct))
    (`EnhancedInputSubsystemInterface.AddMappingContext` (pcsubsystem `EnhancedInputLocalPlayerSubsystem` (`GameplayStatics.GetPlayerController` 0)) (`self.Character Mapping Context`) 2 (struct))))

(fn `Interact`
  (params (`Player Character` :type "/Game/BPs/Player/BP_FirstPersonCharacter Object Reference") (PickUpItem :type "/Game/BPs/PickUps/BP_PickUpItem Object Reference"))
  (returns (UsedPickUp :type Boolean))
  (bind _output_get (set `self.Player HUD` (`/Game/BPs/Player/BP_FirstPersonCharacter.PlayerHUD` `Player Character`)))
  (`/Game/UI/Player/BPW_PlayerHUD.Un/hide HUD` _output_get true)
  (`self.Read`)
  (return false))

(fn `UserConstructionScript`)