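; BP_Clue is an interactable clue that shows readable note text, plays dialogue, or both, with its clue type displayed on a text render.
; Interact checks the GameInstance's Clues map, marking a listed clue as seen or switching to already-seen dialogue.
; With HasRead set, it opens a note widget and swaps input mappings; closing restores controls, then starts any dialogue.
; DestroyAfterInteract destroys the actor when the dialogue component's widget is destroyed.
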(event `self.ReceiveBeginPlay`
  (`TextRenderComponent.K2_SetText` (`self.TextRender`) (`KismetTextLibrary.Conv_StringToText` (`|GetEnumeratorNameAsString` (`self.Clue_type`))))
  (if (`self.DestroyAfterInteract`)
    (add `/Game/BPs/BP_ItemDialogueComp.Widget Destroyed` (`self.BP_ItemDialogueComp`) (delegate `Destroy`))))

(event `Destroy`
  (`self.K2_DestroyActor`))

(event `ReadNote`
  (set `PlayerController.bShowMouseCursor` true (`GameplayStatics.GetPlayerController` 0))
  (`EnhancedInputSubsystemInterface.RemoveMappingContext` (pcsubsystem `EnhancedInputLocalPlayerSubsystem` (`GameplayStatics.GetPlayerController` 0)) (`self.Character Mapping Context`) (struct))
  (`EnhancedInputSubsystemInterface.AddMappingContext` (pcsubsystem `EnhancedInputLocalPlayerSubsystem` (`GameplayStatics.GetPlayerController` 0)) (`self.Mapping Context`) 2 (struct))
  (bind _returnvalue (`|CreateWidget` "/Game/UI/PaperNotes/BPW_ReadableNoteLong.BPW_ReadableNoteLong_C" null (`self.Text to Read`) (`self.Show Header Notification?`) self (`self.HeaderTitle`) (`self.Diff Header Title?`)))
  (bind _output_get (set `self.ReadWidget` _returnvalue))
  (`UserWidget.AddToViewport` _output_get 0)
  (`WidgetBlueprintLibrary.SetInputMode_GameAndUIEx` (`GameplayStatics.GetPlayerController` 0) _output_get "DoNotLock" true true)
  (add `/Game/UI/PaperNotes/BPW_ReadableNoteLong.Close` _returnvalue (delegate `CloseButton`)))

(event `CloseButton`
  (bind _returnvalue (`GameplayStatics.GetPlayerController` 0))
  (set `PlayerController.bShowMouseCursor` false _returnvalue)
  (`WidgetBlueprintLibrary.SetInputMode_GameOnly` _returnvalue true)
  (`Widget.RemoveFromParent` (`self.ReadWidget`))
  (`/Game/UI/Player/BPW_PlayerHUD.Un/hide HUD` (`/Game/BPs/Player/BP_FirstPersonCharacter.PlayerHUD` (`self.Player Character`)) false)
  (`EnhancedInputSubsystemInterface.RemoveMappingContext` (pcsubsystem `EnhancedInputLocalPlayerSubsystem` (`GameplayStatics.GetPlayerController` 0)) (`self.Mapping Context`) (struct))
  (`EnhancedInputSubsystemInterface.AddMappingContext` (pcsubsystem `EnhancedInputLocalPlayerSubsystem` (`GameplayStatics.GetPlayerController` 0)) (`self.Character Mapping Context`) 2 (struct))
  (`KismetSystemLibrary.DelayUntilNextTick`)
  (`/Engine/EditorBlueprintResources/StandardMacros.IsValid` (`self.Dialogue`)
    (:`Is Valid`
      (`self.Set Dialogue`))))

(fn `CheckClueType`
  (bind _asbp_game_instance (cast `/Game/Game_mode-Game_instance/BP_GameInstance` (`GameplayStatics.GetGameInstance`)))
  (bind (_value _returnvalue) (`BlueprintMapLibrary.Map_Find` (`/Game/Game_mode-Game_instance/BP_GameInstance.Clues` _asbp_game_instance) (`self.Clue_type`)))
  (if _returnvalue
    (if _value
      (set `self.Dialogue` (`self.AlreadySawDT`))
      (else
        (`BlueprintMapLibrary.Map_Add` (`/Game/Game_mode-Game_instance/BP_GameInstance.Clues` _asbp_game_instance) (`self.Clue_type`) true)))))

(fn `Interact`
  (params (`Player Character` :type "/Game/BPs/Player/BP_FirstPersonCharacter Object Reference") (PickUpItem :type "/Game/BPs/PickUps/BP_PickUpItem Object Reference"))
  (returns (UsedPickUp :type Boolean))
  (set `self.Player Character` `Player Character`)
  (`self.CheckClueType`)
  (if (`self.HasRead?`)
    (`/Game/UI/Player/BPW_PlayerHUD.Un/hide HUD` (`/Game/BPs/Player/BP_FirstPersonCharacter.PlayerHUD` `Player Character`) true)
    (`self.ReadNote`)
    (else
      (`/Engine/EditorBlueprintResources/StandardMacros.IsValid` (`self.Dialogue`)
        (:`Is Valid`
          (`self.Set Dialogue`)))))
  (return false))

(fn `Set Dialogue`
  (bind _bp_itemdialoguecomp (`self.BP_ItemDialogueComp`))
  (set `/Game/BPs/BP_ItemDialogueComp.Dialogue Data Table` (`self.Dialogue`) _bp_itemdialoguecomp)
  (`/Game/BPs/BP_ItemDialogueComp.StartInteractDialogue` _bp_itemdialoguecomp))

(fn `UserConstructionScript`)