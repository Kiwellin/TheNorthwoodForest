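; BP_PickUpClue is an interactable clue pickup that marks its clue type as found when the player interacts with it.
; On BeginPlay, its TextRender displays the ClueType enum name.
; Interact calls the parent implementation, then CheckClueType flips that type's entry in the BP_GameInstance Clues map from false to true.
; Clue types absent from the map are ignored, and Interact always returns false.
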(event `self.ReceiveBeginPlay`
  (`TextRenderComponent.K2_SetText` (`self.TextRender`) (`KismetTextLibrary.Conv_StringToText` (`|GetEnumeratorNameAsString` (`self.Clue_type`)))))

(fn `CheckClueType`
  (bind _asbp_game_instance (cast `/Game/Game_mode-Game_instance/BP_GameInstance` (`GameplayStatics.GetGameInstance`)))
  (bind (_value _returnvalue) (`BlueprintMapLibrary.Map_Find` (`/Game/Game_mode-Game_instance/BP_GameInstance.Clues` _asbp_game_instance) (`self.Clue_type`)))
  (if _returnvalue
    (if (not _value)
      (`BlueprintMapLibrary.Map_Add` (`/Game/Game_mode-Game_instance/BP_GameInstance.Clues` _asbp_game_instance) (`self.Clue_type`) true))))

(fn `Interact`
  (params (`Player Character` :type "/Game/BPs/Player/BP_FirstPersonCharacter Object Reference") (PickUpItem :type "/Game/BPs/PickUps/BP_PickUpItem Object Reference"))
  (returns (UsedPickUp :type Boolean))
  (`parent.Interact` `Player Character` PickUpItem)
  (set `self.Player Character` null)
  (`self.CheckClueType`)
  (return false))

(fn `UserConstructionScript`)