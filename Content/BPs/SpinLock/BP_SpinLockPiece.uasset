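; Rotating piece of a spin lock that steps through numbered positions and animates to the selected one.
; MoveUpDown shifts the number one step, wraps it around the index list, derives an evenly spaced target roll and returns the number.
; A looping timer runs RotatePiece, which lerps the relative roll along the shortest path and clears itself once the roll exactly equals the target.
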(fn `Clamp`
  (`|ExecutionSequence`
    (:`then_0`
      (if (> (`self.Number`) (`KismetArrayLibrary.Array_LastIndex` (`self.NumberIndex`)))
        (set `self.Number` (- (`self.Number`) (`KismetArrayLibrary.Array_Length` (`self.NumberIndex`))))))
    (:`then_1`
      (if (< (`self.Number`) 0)
        (set `self.Number` (+ (`self.Number`) (`KismetArrayLibrary.Array_Length` (`self.NumberIndex`))))))))

(fn `MoveUpDown`
  (params (Up :type Boolean))
  (returns (Number :type Integer))
  (bind _number (`self.Number`))
  (set `self.Number` (+ (`self.Number`) (`KismetMathLibrary.SelectInt` 1 -1 Up)))
  (`self.Clamp`)
  (set `self.TargetRotation` (* (`self.Number`) (/ 360.0 (`KismetMathLibrary.Conv_IntToDouble` (`KismetArrayLibrary.Array_Length` (`self.NumberIndex`))))))
  (bind _returnvalue (`KismetSystemLibrary.K2_SetTimer` null "RotatePiece" 0.02 true))
  (set `self.Timer` _returnvalue)
  (set `self.Label` (`KismetStringLibrary.Conv_IntToString` _number))
  (return _number))

(fn `RotatePiece`
  (bind _relativerotation_roll (`KismetMathLibrary.BreakRotator` (`self.RelativeRotation`)))
  (`self.K2_SetRelativeRotation` (`KismetMathLibrary.RLerp` (`self.RelativeRotation`) (`KismetMathLibrary.MakeRotator` (`self.TargetRotation`)) (* (`GameplayStatics.GetWorldDeltaSeconds`) 15.0) true))
  (if (== _relativerotation_roll (`self.TargetRotation`))
    (`KismetSystemLibrary.K2_ClearAndInvalidateTimerHandle` (`self.Timer`))))