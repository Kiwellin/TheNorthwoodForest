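; BP_SpinLockPawn is a possessable spin-lock puzzle pawn with four pieces, where the player dials in a code.
; Left and right input cycles the selection with wraparound, marked by an overlay highlight material that clears on returning to the character.
; Up and down input moves the selected piece and writes its label into a comma-delimited code string.
; A match with the correct code, commas stripped, calls PlaySolved.
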(event `self.ReceiveBeginPlay`
  (`parent.ReceiveBeginPlay`)
  (set `self.SpinLockPieces` (`|MakeArray` (`self.BP_SpinLockPiece1`) (`self.BP_SpinLockPiece2`) (`self.BP_SpinLockPiece3`) (`self.BP_SpinLockPiece4`))))

(event `EnhancedInput|/Game/Input/Actions/IA_ExitPuzzle`
  (params (ActionValue :type Boolean) (ElapsedSeconds :type "Float (double-precision)") (TriggeredSeconds :type "Float (double-precision)") (InputAction :type "InputAction Object Reference" :default "/Game/Input/Actions/IA_ExitPuzzle.IA_ExitPuzzle"))
  (:`Triggered`
    (`self.ReturnToCharacter`)))

(event `self.GetPossessed`
  (`parent.GetPossessed`)
  (`self.UpdateHighlightOfSelectedPiece` true))

(event `self.ReturnToCharacter`
  (`parent.ReturnToCharacter`)
  (`self.UpdateHighlightOfSelectedPiece` false))

(event `EnhancedInput|/Game/Input/Actions/IA_NavigateRight`
  (params (ActionValue :type Boolean) (ElapsedSeconds :type "Float (double-precision)") (TriggeredSeconds :type "Float (double-precision)") (InputAction :type "InputAction Object Reference" :default "/Game/Input/Actions/IA_NavigateRight.IA_NavigateRight"))
  (:`Triggered`
    (`self.NavigatePieces` 1)))

(event `EnhancedInput|/Game/Input/Actions/IA_NavigateLeft`
  (params (ActionValue :type Boolean) (ElapsedSeconds :type "Float (double-precision)") (TriggeredSeconds :type "Float (double-precision)") (InputAction :type "InputAction Object Reference" :default "/Game/Input/Actions/IA_NavigateLeft.IA_NavigateLeft"))
  (:`Triggered`
    (`self.NavigatePieces` -1)))

(event `EnhancedInput|/Game/Input/Actions/IA_NavigateUp`
  (params (ActionValue :type Boolean) (ElapsedSeconds :type "Float (double-precision)") (TriggeredSeconds :type "Float (double-precision)") (InputAction :type "InputAction Object Reference" :default "/Game/Input/Actions/IA_NavigateUp.IA_NavigateUp"))
  (:`Triggered`
    (`/Game/BPs/SpinLock/BP_SpinLockPiece.MoveUpDown` (`self.GetSelectedPiece`) true)
    (`self.ChangeDisplay`)))

(event `EnhancedInput|/Game/Input/Actions/IA_NavigateDown`
  (params (ActionValue :type Boolean) (ElapsedSeconds :type "Float (double-precision)") (TriggeredSeconds :type "Float (double-precision)") (InputAction :type "InputAction Object Reference" :default "/Game/Input/Actions/IA_NavigateDown.IA_NavigateDown"))
  (:`Triggered`
    (`/Game/BPs/SpinLock/BP_SpinLockPiece.MoveUpDown` (`self.GetSelectedPiece`) false)
    (`self.ChangeDisplay`)))

(fn `ChangeDisplay`
  (bind _output_get (set `self.CodeArray` (`KismetStringLibrary.ParseIntoArray` (`self.Code`) ",")))
  (`KismetArrayLibrary.Array_Set` _output_get (`self.CurrentPieceIndex`) (`/Game/BPs/SpinLock/BP_SpinLockPiece.Label` (`|GetArrayItem` (`self.SpinLockPieces`) (`self.CurrentPieceIndex`))))
  (set `self.Code` "")
  (for _array_element (`self.CodeArray`)
    (set `self.Code` (`KismetStringLibrary.Concat_StrStr` (`self.Code`) (`KismetStringLibrary.Concat_StrStr` _array_element ","))))
  (if (`self.IsCodeCorrect`)
    (`self.PlaySolved`)))

(fn `GetSelectedPiece`
  (returns (Output :type "/Game/BPs/SpinLock/BP_SpinLockPiece Object Reference"))
  (return (`|GetArrayItem` (`self.SpinLockPieces`) (`self.CurrentPieceIndex`))))

(fn `Interact`
  (params (`Player Character` :type "/Game/BPs/Player/BP_FirstPersonCharacter Object Reference") (PickUpItem :type "/Game/BPs/PickUps/BP_PickUpItem Object Reference"))
  (returns (UsedPickUp :type Boolean))
  (bind _usedpickup (`parent.Interact` `Player Character` PickUpItem))
  (return _usedpickup))

(fn `IsCodeCorrect`
  (returns (ReturnValue :type Boolean))
  (return (`KismetStringLibrary.EqualEqual_StrStr` (`self.CorrectCode`) (`KismetStringLibrary.Replace` (`self.Code`) ","))))

(fn `NavigatePieces`
  (params (Direction :type Integer))
  (`self.UpdateHighlightOfSelectedPiece` false)
  (set `self.CurrentPieceIndex` (+ (`self.CurrentPieceIndex`) Direction))
  (`|ExecutionSequence`
    (:`then_0`
      (if (> (`self.CurrentPieceIndex`) (`KismetArrayLibrary.Array_LastIndex` (`self.SpinLockPieces`)))
        (set `self.CurrentPieceIndex` (- (`self.CurrentPieceIndex`) (`KismetArrayLibrary.Array_Length` (`self.SpinLockPieces`))))))
    (:`then_1`
      (if (< (`self.CurrentPieceIndex`) 0)
        (set `self.CurrentPieceIndex` (+ (`self.CurrentPieceIndex`) (`KismetArrayLibrary.Array_Length` (`self.SpinLockPieces`))))))
    (:`then_2`
      (`self.UpdateHighlightOfSelectedPiece` true))))

(fn `UpdateHighlightOfSelectedPiece`
  (params (Enable :type Boolean))
  (`MeshComponent.SetOverlayMaterial` (`self.GetSelectedPiece`) (select `bool` Enable :`true` "/Game/Materials/placeholder/MI_HighlightSpinlock.MI_HighlightSpinlock" :!type "MaterialInterface Object Reference")))

(fn `UserConstructionScript`
  (`parent.UserConstructionScript`))