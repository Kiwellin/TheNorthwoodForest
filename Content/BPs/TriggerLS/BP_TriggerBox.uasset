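; BP_TriggerBox is a one-shot trigger that starts a level sequence cutscene with dialogue when the first-person character enters it.
; On overlap it destroys the box, plays LS, shows a data-table-driven dialogue widget and disables input.
; When dialogue ends, a camera fade covers stopping the sequence, optionally teleporting the player to Cube, and restoring control.
; An optional follow-up dialogue then locks input again, with event dispatchers announcing each stage.
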(event `self.Box.OnComponentBeginOverlap`
  (params (OverlappedComponent :type "PrimitiveComponent Object Reference") (OtherActor :type "Actor Object Reference") (OtherComp :type "PrimitiveComponent Object Reference") (OtherBodyIndex :type Integer) (bFromSweep :type Boolean) (SweepResult :type "HitResult Structure (by ref)"))
  (bind _asbp_first_person_character (cast `/Game/BPs/Player/BP_FirstPersonCharacter` OtherActor))
  (`/Engine/EditorBlueprintResources/StandardMacros.DoOnce` false
    (:`Completed`
      (`ActorComponent.K2_DestroyComponent` (`self.Box`))
      (`/Engine/EditorBlueprintResources/StandardMacros.IsValid` (`self.LS`)
        (:`Is Valid`
          (`MovieSceneSequencePlayer.Play` (`LevelSequenceActor.SequencePlayer` (`self.LS`)))
          (`self.StartedCutscene`)
          (`self.SequenceStart` _asbp_first_person_character)
          (add `/Game/UI/Dialogue/BPW_Dialogue.CallEnded` (`self.DialogueWidget`) (delegate `Remove Widget`))
          (`self.DisableInput` (`GameplayStatics.GetPlayerPawn` 0) (`GameplayStatics.GetPlayerController` 0)))))))

(event `Remove Widget`
  (bind (_returnvalue_location _returnvalue_rotation) (`KismetMathLibrary.BreakTransform` (`SceneComponent.K2_GetComponentToWorld` (`self.Cube`))))
  (`Widget.RemoveFromParent` (`self.DialogueWidget`))
  (set `self.DialogueWidget` null)
  (`PlayerCameraManager.StartCameraFade` :`self` (`GameplayStatics.GetPlayerCameraManager` 0) :`ToAlpha` 1.0 :`Duration` 1.0 :`bHoldWhenFinished` true)
  (`KismetSystemLibrary.Delay` 1.0)
  (bind _asbp_first_person_character (cast `/Game/BPs/Player/BP_FirstPersonCharacter` (`GameplayStatics.GetPlayerCharacter` 0)))
  (if (`self.Teleport?`)
    (`Controller.SetControlRotation` (`GameplayStatics.GetPlayerController` 0) _returnvalue_rotation)
    (`self.K2_SetActorTransform` _asbp_first_person_character (`KismetMathLibrary.MakeTransform` _returnvalue_location) false false)
    (`KismetSystemLibrary.Delay` 1.0))
  (`/Game/UI/Player/BPW_PlayerHUD.Un/hide HUD` (`/Game/BPs/Player/BP_FirstPersonCharacter.PlayerHUD` _asbp_first_person_character) false)
  (`MovieSceneSequencePlayer.Stop` (`LevelSequenceActor.SequencePlayer` (`self.LS`)))
  (`self.EnableInput` (`GameplayStatics.GetPlayerPawn` 0) (`GameplayStatics.GetPlayerController` 0))
  (`ActorComponent.Activate` (`/Game/BPs/Player/BP_FirstPersonCharacter.Camera` _asbp_first_person_character) false)
  (`PlayerCameraManager.StartCameraFade` :`self` (`GameplayStatics.GetPlayerCameraManager` 0) :`FromAlpha` 1.0 :`Duration` 1.0)
  (`self.CutsceneEnd`)
  (`/Engine/EditorBlueprintResources/StandardMacros.IsValid` (`self.WidgetAfterLS`)
    (:`Is Valid`
      (bind _returnvalue (`|CreateWidget` "/Game/UI/Dialogue/BPW_Dialogue.BPW_Dialogue_C"))
      (bind _output_get (set `self.DialogueWidget` _returnvalue))
      (set `/Game/UI/Dialogue/BPW_Dialogue.DialogueDataTable` (`self.WidgetAfterLS`) _output_get)
      (`UserWidget.AddToViewport` (`self.DialogueWidget`) 0)
      (add `/Game/UI/Dialogue/BPW_Dialogue.CallEnded` (`self.DialogueWidget`) (delegate `EndDialogue`))
      (`self.DisableInput` (`GameplayStatics.GetPlayerPawn` 0) (`GameplayStatics.GetPlayerController` 0)))))

(event `EndDialogue`
  (`Widget.RemoveFromParent` (`self.DialogueWidget`))
  (set `self.DialogueWidget` null)
  (`self.EnableInput` (`GameplayStatics.GetPlayerPawn` 0) (`GameplayStatics.GetPlayerController` 0))
  (`self.SecondDialogueEnd`))

(fn `SequenceStart`
  (params (FirstPersonCharacter :type "/Game/BPs/Player/BP_FirstPersonCharacter Object Reference"))
  (`/Game/UI/Player/BPW_PlayerHUD.Un/hide HUD` (`/Game/BPs/Player/BP_FirstPersonCharacter.PlayerHUD` FirstPersonCharacter) true)
  (`/Engine/EditorBlueprintResources/StandardMacros.IsValid` (`self.DialogueWidget`)
    (:`Is Not Valid`
      (bind _returnvalue (`|CreateWidget` "/Game/UI/Dialogue/BPW_Dialogue.BPW_Dialogue_C"))
      (bind _output_get (set `self.DialogueWidget` _returnvalue))
      (set `/Game/UI/Dialogue/BPW_Dialogue.DialogueDataTable` (`self.Dialogue Data Table`) _output_get)
      (`UserWidget.AddToViewport` (`self.DialogueWidget`) 0))))

(fn `UserConstructionScript`)