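; Player controller that manages which Enhanced Input mapping context is active for first-person play and the notebook.
; On BeginPlay it adds the first-person context to the local player's Enhanced Input subsystem.
; The IMCNotebookSwitch event takes an open flag and swaps between the first-person and notebook contexts, removing one before adding the other at the same priority.
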(event `self.ReceiveBeginPlay`
  (`EnhancedInputSubsystemInterface.AddMappingContext` (subsystem `EnhancedInputLocalPlayerSubsystem`) (`self.FirstPersonIMC`) 0 (struct)))

(event `IMCNotebookSwitch`
  (params (`OpenNoteBook?` :type Boolean))
  (bind _returnvalue (subsystem `EnhancedInputLocalPlayerSubsystem`))
  (bind _returnvalue_2 (subsystem `EnhancedInputLocalPlayerSubsystem`))
  (if `OpenNoteBook?`
    (`EnhancedInputSubsystemInterface.RemoveMappingContext` _returnvalue_2 (`self.FirstPersonIMC`) (struct))
    (`EnhancedInputSubsystemInterface.AddMappingContext` _returnvalue_2 (`self.NoteBookIMC`) 0 (struct))
    (else
      (`EnhancedInputSubsystemInterface.RemoveMappingContext` _returnvalue (`self.NoteBookIMC`) (struct))
      (`EnhancedInputSubsystemInterface.AddMappingContext` _returnvalue (`self.FirstPersonIMC`) 0 (struct)))))

(fn `UserConstructionScript`)