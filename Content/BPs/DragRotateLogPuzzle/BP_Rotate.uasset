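; Rotatable piece for the drag-rotate log puzzle, limiting how far its static mesh can turn.
; While ClampRotate is above zero, Tick clamps the mesh's world yaw to a fixed arc, zeroes pitch and roll, and prints the rotation for debugging.
; The dragging itself is not handled here, and a note marks the per-tick clamp as provisional, to move to a timer.
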(event `self.ReceiveTick`
  (params (DeltaSeconds :type "Float (single-precision)"))
  (bind _staticmesh (`self.StaticMesh`))
  (bind (_returnvalue_roll _returnvalue_pitch _returnvalue_yaw) (`KismetMathLibrary.BreakRotator` (`SceneComponent.K2_GetComponentRotation` (`self.StaticMesh`))))
  (`parent.ReceiveTick` DeltaSeconds)
  ; Clamp rotation , put boolean for optional, put on a timer instead. ALSO!? Maybe use branch as component check in player to check from whcih side u can pull?
  (if (> (`self.ClampRotate`) 0.0)
    (`SceneComponent.K2_SetWorldRotation` _staticmesh (`KismetMathLibrary.MakeRotator` 0.0 0.0 (`KismetMathLibrary.ClampAngle` _returnvalue_yaw 0.0 45.0)) false false)
    (`KismetSystemLibrary.PrintString` (`KismetStringLibrary.Conv_RotatorToString` (`SceneComponent.K2_GetComponentRotation` _staticmesh)))))

(fn `UserConstructionScript`
  (`parent.UserConstructionScript`))