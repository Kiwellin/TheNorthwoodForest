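; Interactable rotating stone for the animal audio puzzle that turns in 90-degree steps toward a correct yaw.
; Interacting picks the turn direction from whether the stone sits left or right of the camera's view center, updates the wrapped target yaw and plays a sound.
; Tick smoothly lerps the mesh to that yaw.
; After a short delay, the GiveRotationBool dispatcher broadcasts whether the rotation is correct.
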(event `self.ReceiveBeginPlay`
  (bind (_relativerotation_roll _relativerotation_pitch _relativerotation_yaw) (`KismetMathLibrary.BreakRotator` (`SceneComponent.RelativeRotation` (`self.StaticMesh`))))
  (set `self.TargetRotation` _relativerotation_yaw))

(event `Turn`
  (`self.Get RotationDirection`)
  (`self.SetTargetRotation`)
  (`GameplayStatics.PlaySound2D` "/Game/Audio/SFX/AnimalStones/SC_Stoneturn.SC_Stoneturn" 1.0 1.0 0.0 null null)
  (`KismetSystemLibrary.Delay` 0.2)
  (bind _is_correct (`self.CheckIfCorrect`))
  (bind _output_get (set `self.Is Correct` _is_correct))
  (`self.GiveRotationBool` _output_get self))

(event `self.ReceiveTick`
  (params (DeltaSeconds :type "Float (single-precision)"))
  (`SceneComponent.K2_SetRelativeRotation` (`self.StaticMesh`) (`KismetMathLibrary.RLerp` (`SceneComponent.RelativeRotation` (`self.StaticMesh`)) (`KismetMathLibrary.MakeRotator` 0.0 0.0 (`self.TargetRotation`)) (* (`GameplayStatics.GetWorldDeltaSeconds`) 15.0) true) false false))

(fn `CheckIfCorrect`
  (returns (`Is Correct` :type Boolean))
  (if (== (`self.TargetRotation`) (`self.CorrectRotation`))
    (return true)
    (else
      (return false))))

(fn `Get RotationDirection`
  (bind (_location _rotation) (`Controller.GetPlayerViewPoint` (`GameplayStatics.GetPlayerController` 0)))
  (if (> (`KismetMathLibrary.Dot_VectorVector` (`KismetMathLibrary.Vector_Normal2D` (- (`self.K2_GetActorLocation`) _location)) (`KismetMathLibrary.Vector_Normal2D` (`KismetMathLibrary.GetRightVector` _rotation))) 0.0)
    (set `self.RotDirection` 1.0)
    (else
      (set `self.RotDirection` -1.0)))
  (return))

(fn `Interact`
  (params (`Player Character` :type "/Game/BPs/Player/BP_FirstPersonCharacter Object Reference") (PickUpItem :type "/Game/BPs/PickUps/BP_PickUpItem Object Reference"))
  (returns (UsedPickUp :type Boolean))
  (if (`self.CanBeInteractedWith`)
    (`self.Turn`)
    (return false)))

(fn `SetTargetRotation`
  (bind _returnvalue (+ (`self.TargetRotation`) (* 90.0 (`self.RotDirection`))))
  (`|ExecutionSequence`
    (:`then_0`
      (if (> _returnvalue 360.0)
        (set `self.TargetRotation` 0.0)))
    (:`then_1`
      (if (< _returnvalue 0.0)
        (set `self.TargetRotation` 360.0)))
    (:`then_2`
      (bind _output_get (set `self.TargetRotation` _returnvalue))
      (if (or (== _output_get 0.0) (== _output_get 360.0))
        (set `self.TargetRotation` 0.0)
        (else
          (`KismetSystemLibrary.PrintString` (`KismetStringLibrary.Conv_DoubleToString` (`self.TargetRotation`))))))))

(fn `UserConstructionScript`)