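; BP_AnimalSound is an animal sound emitter for the animal audio puzzle, playing its Audio component either as a loop or at random intervals.
; When IsLoopedAudio is set, BeginPlay starts the audio once through a DoOnce.
; Otherwise, a timer fires the Play event after a random delay of several seconds, and each play schedules the next with a new random delay.
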(event `self.ReceiveBeginPlay`
  (if (`self.IsLoopedAudio?`)
    (`/Engine/EditorBlueprintResources/StandardMacros.DoOnce` false
      (:`Completed`
        (`AudioComponent.Play` (`self.Audio`) 0.0)))
    (else
      (set `self.Time` (`KismetMathLibrary.RandomFloatInRange` 4.0 15.0))
      (`KismetSystemLibrary.K2_SetTimerDelegate` (delegate `Play`) (`self.Time`)))))

(event `Play`
  (`AudioComponent.Play` (`self.Audio`) 0.0)
  (bind _output_get (set `self.Time` (`KismetMathLibrary.RandomFloatInRange` 4.0 15.0)))
  (`KismetSystemLibrary.K2_SetTimerDelegate` (delegate `Play`) _output_get))

(fn `UserConstructionScript`)