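; BP_Gate is a gate actor that swings open when its linked button or puzzle signals it.
; On BeginPlay it binds OpenGate to the assigned Button, or to the assigned Puzzle's solved event if no valid Button is set.
; OpenGate plays a timeline that lerps the mesh's relative rotation from zero to OpenAmount on a roll, pitch or yaw axis chosen by the Rotation setting.
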(event `self.ReceiveBeginPlay`
  (bind _button (`self.Button`))
  (bind _puzzle (`self.Puzzle`))
  (`/Engine/EditorBlueprintResources/StandardMacros.IsValid` _button
    (:`Is Valid`
      (add `/Game/BPs/GateAndButton/BP_ButtonGate.OpenGate` _button (delegate `OpenGate`)))
    (:`Is Not Valid`
      (`/Engine/EditorBlueprintResources/StandardMacros.IsValid` _puzzle
        (:`Is Valid`
          (add `/Game/BPs/InteractablePossessables/BP_InteractablePossessable.SolvedPuzzle` _puzzle (delegate `OpenGate`)))))))

(event `OpenGate`
  (bind (_direction _rotate) (`Timeline|Open` :!via `PlayFromStart`)
    (:`Update`
      (switch `int` (`self.Rotation`)
        (:`1`
          (bind _returnvalue (`KismetMathLibrary.Lerp` 0.0 (`self.OpenAmount`) _rotate))
          (`SceneComponent.K2_SetRelativeRotation` (`self.StaticMesh`) (`KismetMathLibrary.MakeRotator` _returnvalue) false false))
        (:`2`
          (`SceneComponent.K2_SetRelativeRotation` (`self.StaticMesh`) (`KismetMathLibrary.MakeRotator` 0.0 _returnvalue) false false))
        (:`3`
          (`SceneComponent.K2_SetRelativeRotation` (`self.StaticMesh`) (`KismetMathLibrary.MakeRotator` 0.0 0.0 _returnvalue) false false))))))

(fn `UserConstructionScript`)