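; BP_ButtonGate is an interactable button that opens a gate once it has electricity.
; Solving the CableConnect ports powers it, swapping the sphere's material and the point light's color.
; Interact plays a timeline that pushes the sphere in, plays a sound and reverses, with a flag blocking overlapping presses.
; The first completed powered press calls OpenGate and disables further presses; unpowered presses only animate and click.
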(event `self.ReceiveBeginPlay`
  (add `/Game/BPs/InteractablePossessables/BP_CableConnect.SolvedPorts` (`self.CableConnect`) (delegate `SetMaterial`))
  (`TimelineComponent.SetPlayRate` (`self.PressButton`) 2.0))

(event `SetMaterial`
  (`PrimitiveComponent.SetMaterial` (`self.Sphere`) 0 (`self.ActivateMaterial`))
  (`LightComponent.SetLightColor` (`self.PointLight`) (`self.ActiveLightColor`) true)
  (set `self.HasElectricity` true))

(event `TryActivate`
  (bind _pressbutton (`self.PressButton`))
  (bind _buttonrelative_location_x (`KismetMathLibrary.BreakVector` (`self.ButtonRelative Location`)))
  (if (not (`self.PressedButton`))
    (set `self.PressedButton` true)
    (set `self.ButtonRelative Location` (`SceneComponent.RelativeLocation` (`self.Sphere`)))
    (bind (_direction _pressdirection) (`Timeline|PressButton` :!via `PlayFromStart` :!label _label)
      (:`Update`
        (`SceneComponent.K2_SetRelativeLocation` (`self.Sphere`) (`KismetMathLibrary.MakeVector` (`KismetMathLibrary.Lerp` _buttonrelative_location_x (+ _buttonrelative_location_x 10.0) _pressdirection)) false false))
      (:`Finished`
        (if (== (`TimelineComponent.GetPlaybackPosition` _pressbutton) (`TimelineComponent.GetTimelineLength` _pressbutton))
          (`self.PlayBack`)
          (`GameplayStatics.PlaySound2D` "/Game/Audio/SFX/Ui/SC_PhoneDialogueButton.SC_PhoneDialogueButton" 1.0 1.0 0.0 null null)
          (if (`self.HasElectricity`)
            (`/Engine/EditorBlueprintResources/StandardMacros.DoOnce` false
              (:`Completed`
                (set `self.CanBePressed` false)
                (`self.OpenGate`))))
          (else
            (set `self.PressedButton` false)))))))

(event `PlayBack`
  (goto _label :!via `ReverseFromEnd`))

(fn `Interact`
  (params (`Player Character` :type "/Game/BPs/Player/BP_FirstPersonCharacter Object Reference") (PickUpItem :type "/Game/BPs/PickUps/BP_PickUpItem Object Reference"))
  (returns (UsedPickUp :type Boolean))
  (if (`self.CanBePressed`)
    (`self.TryActivate`))
  (return false))

(fn `UserConstructionScript`)