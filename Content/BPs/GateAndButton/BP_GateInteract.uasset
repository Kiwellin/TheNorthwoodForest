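; An interactable gate that rotates open, either with a matching key item or through a plain interaction.
; Interact compares the picked-up item to Key when NeedsKey is set, returning true on a match; keyless gates with a box component destroy it, open and return false.
; OpenGate plays a timeline that lerps the static mesh's relative rotation to OpenAmount on the axis selected by Rotation.
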(event `self.ReceiveBeginPlay`
  (bind _output_get (set `self.BoxCol` (`self.GetComponentByClass` "/Script/Engine.BoxComponent")))
  (`/Engine/EditorBlueprintResources/StandardMacros.IsValid` _output_get
    (:`Is Valid`
      (set `self.InteractionBox` true))))

(event `OpenGate`
  (bind (_direction _rotate) (`Timeline|Open` :!via `PlayFromStart`)
    (:`Update`
      (switch `int` (`self.Rotation`)
        (:`1`
          (bind _returnvalue (`KismetMathLibrary.Lerp` 0.0 (`self.OpenAmount`) _rotate))
          (`SceneComponent.K2_SetRelativeRotation` (`self.StaticMesh`) (`KismetMathLibrary.MakeRotator` _returnvalue) false false))
        (:`2`
          (`SceneComponent.K2_SetRelativeRotation` (`self.StaticMesh`) (`KismetMathLibrary.MakeRotator` 0.0 _returnvalue) false false))
        (:`3`
          (`SceneComponent.K2_SetRelativeRotation` (`self.StaticMesh`) (`KismetMathLibrary.MakeRotator` 0.0 0.0 _returnvalue) false false))))))

(fn `Interact`
  (params (`Player Character` :type "/Game/BPs/Player/BP_FirstPersonCharacter Object Reference") (PickUpItem :type "/Game/BPs/PickUps/BP_PickUpItem Object Reference"))
  (returns (UsedPickUp :type Boolean))
  (if (`self.NeedsKey`)
    (if (== (`self.Key`) PickUpItem)
      (`self.OpenGate`)
      (set `self.NeedsKey` false)
      (return true))
    (elif (`self.InteractionBox`)
      (`ActorComponent.K2_DestroyComponent` (`self.BoxCol`))
      (`self.OpenGate`)
      (set `self.InteractionBox` false)
      (return false))))

(fn `UserConstructionScript`)