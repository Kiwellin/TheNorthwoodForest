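; BP_MathTest is a test Blueprint for expressing a random value as a percentage of a base value.
; On BeginPlay it rolls a random integer, converts it to a double, and prints it.
; It then prints the value safely divided by BaseValue and formatted as a percent.
; Unconnected nodes hold alternative percentage formulas and a float random roll; the construction script is empty.
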(event `self.ReceiveBeginPlay`
  (bind _output_get (set `self.Value` (`KismetMathLibrary.Conv_IntToDouble` (`KismetMathLibrary.RandomIntegerInRange` 0 115))))
  (`KismetSystemLibrary.PrintString` (`KismetStringLibrary.Concat_StrStr` "value: " (`KismetStringLibrary.Conv_DoubleToString` _output_get)))
  (`KismetSystemLibrary.PrintString` (`KismetTextLibrary.Conv_TextToString` (`KismetTextLibrary.AsPercent_Float` (`KismetMathLibrary.SafeDivide` (`self.Value`) (`self.BaseValue`)) "HalfToEven"))))

(fn `UserConstructionScript`)