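; BP_ItemDialogueComp opens a dialogue widget for an item interaction and blocks player pawn input while it is shown.
; StartInteractDialogue creates a BPW_Dialogue only if none is active, passes it the DialogueDataTable, adds it to the viewport and binds to its Ended dispatcher.
; When dialogue ends, RemoveWidget removes and clears the widget, restores input and fires the WidgetDestroyed dispatcher.
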(event `StartInteractDialogue`
  (`/Engine/EditorBlueprintResources/StandardMacros.IsValid` (`self.DialogueWidget`)
    (:`Is Not Valid`
      (bind _returnvalue (`|CreateWidget` "/Game/UI/Dialogue/BPW_Dialogue.BPW_Dialogue_C"))
      (bind _output_get (set `self.DialogueWidget` _returnvalue))
      (set `/Game/UI/Dialogue/BPW_Dialogue.DialogueDataTable` (`self.Dialogue Data Table`) _output_get)
      (`UserWidget.AddToViewport` (`self.DialogueWidget`) 0)
      (add `/Game/UI/Dialogue/BPW_Dialogue.CallEnded` (`self.DialogueWidget`) (delegate `RemoveWidget`))
      (`Actor.DisableInput` (`GameplayStatics.GetPlayerPawn` 0) (`GameplayStatics.GetPlayerController` 0)))))

(event `RemoveWidget`
  (`Widget.RemoveFromParent` (`self.DialogueWidget`))
  (set `self.DialogueWidget` null)
  (`Actor.EnableInput` (`GameplayStatics.GetPlayerPawn` 0) (`GameplayStatics.GetPlayerController` 0))
  (`self.Widget Destroyed`))