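; BP_PayPhone is a possessable interactable payphone that starts a dialogue call when possessed.
; Possession plays a dial sound, waits for its duration, then shows a BPW_Dialogue widget fed by StartDataTable, whose call-ended callback returns to the character, restoring game input and removing the widget.
; A phone flagged as first also triggers CampGate's Rested once.
; The table condition check is an unused random-pick placeholder.
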(event `self.ReceiveBeginPlay`
  (`parent.ReceiveBeginPlay`))

(event `self.GetPossessed`
  (`parent.GetPossessed`)
  (if (`self.IsFirstPhone?`)
    (`/Engine/EditorBlueprintResources/StandardMacros.DoOnce` false
      (:`Completed`
        (set `self.IsFirstPhone?` false)
        (`/Game/BPs/Interactables/Tent/BP_Campgates.Rested` (`self.CampGate`)))))
  (`GameplayStatics.PlaySound2D` (`self.DialSound`) 1.0 1.0 0.0 null null)
  (`KismetSystemLibrary.Delay` (`SoundBase.Duration` (`self.DialSound`)))
  (bind _returnvalue (`|CreateWidget` "/Game/UI/Dialogue/BPW_Dialogue.BPW_Dialogue_C"))
  (bind _output_get (set `self.DialogueUIRef` _returnvalue))
  (set `/Game/UI/Dialogue/BPW_Dialogue.DialogueDataTable` (`self.StartDataTable`) _output_get)
  (`UserWidget.AddToViewport` _output_get 0)
  (add `/Game/UI/Dialogue/BPW_Dialogue.CallEnded` (`self.DialogueUIRef`) (delegate `self.ReturnToCharacter`)))

(event `self.ReturnToCharacter`
  (`parent.ReturnToCharacter`)
  (`WidgetBlueprintLibrary.SetInputMode_GameOnly` (`GameplayStatics.GetPlayerController` 0) true)
  (`Widget.RemoveFromParent` (`self.DialogueUIRef`)))

(fn `GetDataTableAfterConditionCheck`
  (returns (DataTable :type "DataTable Object Reference"))
  (return (select `bool` (`KismetMathLibrary.RandomBool`) :!type "DataTable Object Reference")))

(fn `UserConstructionScript`
  (`parent.UserConstructionScript`))