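; Possessable cable-connection puzzle where the player plugs cable ends into eight ports using the mouse cursor.
; Cursor line traces pick up cables, attach each end to a port or return them to the shelf, while a looping timer moves the physics handle with the cursor.
; Correct connections raise a count that, when full, disables possession and signals solved.
; Interacting reveals extra cables once available, otherwise it starts dialogue.
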(event `self.ReceiveBeginPlay`
  (`parent.ReceiveBeginPlay`)
  (set `self.CableXAxisRef` (`KismetMathLibrary.Abs` (.x (.location (`SceneComponent.GetRelativeTransform` (`self.Cable X MoveAxis Ref`))))))
  (bind _output_get (set `self.PortArray` (`|MakeArray` (`self.BP_ConnectPort`) (`self.BP_ConnectPort1`) (`self.BP_ConnectPort2`) (`self.BP_ConnectPort3`) (`self.BP_ConnectPort4`) (`self.BP_ConnectPort5`) (`self.BP_ConnectPort6`) (`self.BP_ConnectPort7`))))
  (set `self.CorrectPorts` (`KismetArrayLibrary.Array_Length` _output_get)))

(event `RemoveFromCount`
  (params (RemoveAmount :type Integer))
  (set `self.CountPorts` (- (`self.CountPorts`) RemoveAmount))
  (`KismetSystemLibrary.PrintString` (`KismetStringLibrary.Concat_StrStr` "remove " (`KismetStringLibrary.Conv_IntToString` RemoveAmount) "points from count ")))

(event `AddToCount`
  (`/Engine/EditorBlueprintResources/StandardMacros.IncrementInt` (`self.CountPorts`)
    (:`  `
      (`KismetSystemLibrary.PrintString` "add 1 point to count")
      (if (== (`self.CorrectPorts`) (`self.CountPorts`))
        (set `self.CanBePossessed?` false)
        (`self.PlaySolved`)
        (`KismetSystemLibrary.Delay` (`self.SmoothPossessDuration`))
        (`self.SolvedPorts`)))))

(event `self.GetPossessed`
  (bind _returnvalue (`GameplayStatics.GetPlayerController` 0))
  (`parent.GetPossessed`)
  (set `PlayerController.bShowMouseCursor` true _returnvalue)
  (`WidgetBlueprintLibrary.SetInputMode_GameAndUIEx` _returnvalue null "DoNotLock" false))

(event `self.ReturnToCharacter`
  (bind _returnvalue (`GameplayStatics.GetPlayerController` 0))
  (`parent.ReturnToCharacter`)
  (set `PlayerController.bShowMouseCursor` false _returnvalue)
  (`WidgetBlueprintLibrary.SetInputMode_GameOnly` _returnvalue true))

(event `CopyMouseLocation`
  (bind (_worldlocation _worlddirection) (`PlayerController.DeprojectMousePositionToWorld` (`GameplayStatics.GetPlayerController` 0)))
  (`PhysicsHandleComponent.SetTargetLocation` (`self.PhysicsHandle`) (+ _worldlocation (* _worlddirection (`self.CableXAxisRef`)))))

(event `Key|AnyKey`
  (params (Key :type "Key Structure"))
  (:`Pressed`
    (if (`KismetInputLibrary.Key_IsGamepadKey` Key)
      _)))

(event `EnhancedInput|/Game/Input/Actions/IA_ExitPuzzle`
  (params (ActionValue :type Boolean) (ElapsedSeconds :type "Float (double-precision)") (TriggeredSeconds :type "Float (double-precision)") (InputAction :type "InputAction Object Reference" :default "/Game/Input/Actions/IA_ExitPuzzle.IA_ExitPuzzle"))
  (:`Triggered`
    (if (not (`self.HasCableInHand`))
      (`self.ReturnToCharacter`))))

(event `EnhancedInput|/Game/Input/Actions/IA_RotateCamera`
  (params (ActionValue :type "Vector2D Structure") (ElapsedSeconds :type "Float (double-precision)") (TriggeredSeconds :type "Float (double-precision)") (InputAction :type "InputAction Object Reference" :default "/Game/Input/Actions/IA_RotateCamera.IA_RotateCamera"))
  (bind (_locationx _locationy) (`PlayerController.GetMousePosition` (`GameplayStatics.GetPlayerController` 0)))
  (:`Triggered`
    (`PlayerController.SetMouseLocation` (`GameplayStatics.GetPlayerController` 0) (`KismetMathLibrary.Round` (+ (* ActionValue_X 10.0) _locationx)) (`KismetMathLibrary.Round` (+ (* ActionValue_Y 10.0) _locationy)))))

(event `EnhancedInput|/Game/Input/Actions/IA_SelectCable`
  (params (ActionValue :type Boolean) (ElapsedSeconds :type "Float (double-precision)") (TriggeredSeconds :type "Float (double-precision)") (InputAction :type "InputAction Object Reference" :default "/Game/Input/Actions/IA_SelectCable.IA_SelectCable"))
  (bind _returnvalue (`self.GetGrabableCablePart`))
  (bind _cable (`self.Cable`))
  (bind (_worldlocation _worlddirection) (`PlayerController.DeprojectMousePositionToWorld` (`GameplayStatics.GetPlayerController` 0)))
  (bind (_starttrans_location _starttrans_rotation) (`KismetMathLibrary.BreakTransform` (`/Game/BPs/CableConnect/BP_Cable.StartTrans` _cable)))
  (:`Triggered`
    (bind (_outhit _returnvalue_2) (`KismetSystemLibrary.LineTraceSingleForObjects` _worldlocation (+ _worldlocation (* _worlddirection 200.0)) (`|MakeArray` "ObjectTypeQuery1" "ObjectTypeQuery2" "ObjectTypeQuery3" "ObjectTypeQuery4" :!type "EObjectTypeQuery Enum") true (select `bool` (`KismetSystemLibrary.IsValid` (`self.Cable`)) :`true` (`|MakeArray` (`self.Cable`) :!type "Actor Object Reference")) "ForDuration" false))
    (if _returnvalue_2
      (bind (_bblockinghit _binitialoverlap _time _distance _location _impactpoint _normal _impactnormal _physmat _hitactor _hitcomponent) (`GameplayStatics.BreakHitResult` _outhit))
      (bind _iscable_ (`self.CheckIfCable` _hitactor))
      (if _iscable_
        (bind (_removedfromports_ _amountremoved) (`/Game/BPs/CableConnect/BP_Cable.CheckForRemovedCorrectPorts` (`self.Cable`)))
        (if _removedfromports_
          (`self.RemoveFromCount` _amountremoved))
        (else
          (bind _asbp_connect_port (cast `/Game/BPs/CableConnect/BP_ConnectPort` _hitcomponent)
            (:`then`
              (set `self.As BP Connect Port` _asbp_connect_port)
              (`/Engine/EditorBlueprintResources/StandardMacros.IsValid` (`self.Cable`)
                (:`Is Valid`
                  (bind _nocableconnected (`/Game/BPs/CableConnect/BP_ConnectPort.CheckCableStatus` (`self.As BP Connect Port`)))
                  (if _nocableconnected
                    (`self.AttachCablePartToPort` _hitcomponent)
                    (bind _wasrightcable (`/Game/BPs/CableConnect/BP_ConnectPort.CheckCorrectCable` (`self.As BP Connect Port`) (`self.Cable`)))
                    (if _wasrightcable
                      (`self.AddToCount`))
                    (bind _iscablestart_ (`/Game/BPs/CableConnect/BP_Cable.FlipCableEnds` (`self.Cable`)))
                    (if _iscablestart_
                      (set `self.Cable` null)
                      (`KismetSystemLibrary.K2_ClearAndInvalidateTimerHandle` (`self.MouseCopyTimer`))
                      (set `self.HasCableInHand` false)
                      (else
                        (`PhysicsHandleComponent.GrabComponentAtLocation` (`self.PhysicsHandle`) _returnvalue "None" (`SceneComponent.K2_GetComponentLocation` _returnvalue))))
                    (else
                      (`KismetSystemLibrary.PrintString` "fakseeee"))))))
            (:`CastFailed`
              (cast `/Game/BPs/CableConnect/BP_CableShelf` _hitactor)
              (if (`self.HasCableInHand`) :!label _label
                (bind (_removedfromports__2 _amountremoved_2) (`/Game/BPs/CableConnect/BP_Cable.CheckForRemovedCorrectPorts` (`self.Cable`)))
                (if _removedfromports__2
                  (`self.RemoveFromCount` _amountremoved_2))
                (`KismetSystemLibrary.K2_ClearAndInvalidateTimerHandle` (`self.MouseCopyTimer`))
                (`self.DetachCableAndSetTransform` _starttrans_rotation _starttrans_location true)
                (`/Game/BPs/CableConnect/BP_Cable.ResetTransform` _cable)
                (set `self.Cable` null)
                (set `self.HasCableInHand` false)))))))))

(event `EnhancedInput|/Game/Input/Actions/IA_DeselectCable`
  (params (ActionValue :type Boolean) (ElapsedSeconds :type "Float (double-precision)") (TriggeredSeconds :type "Float (double-precision)") (InputAction :type "InputAction Object Reference" :default "/Game/Input/Actions/IA_DeselectCable.IA_DeselectCable"))
  (:`Triggered`
    (goto _label)))

(fn `AttachCablePartToPort`
  (params (HitComponent :type "SceneComponent Object Reference"))
  (bind (_returnvalue_x _returnvalue_y _returnvalue_z) (`KismetMathLibrary.BreakVector` (`SceneComponent.K2_GetComponentLocation` HitComponent)))
  (`self.DetachCableAndSetTransform` (`SceneComponent.K2_GetComponentRotation` HitComponent) (`KismetMathLibrary.MakeVector` (+ _returnvalue_x 5.0) _returnvalue_y _returnvalue_z))
  (`/Game/BPs/CableConnect/BP_Cable.AttachedToPort` (`self.Cable`) (`self.As BP Connect Port`) (`self.GetGrabableCablePart`)))

(fn `CheckIfCable`
  (params (Object :type "Object Object Reference"))
  (returns (`IsCable?` :type Boolean))
  (bind _returnvalue (`self.GetGrabableCablePart`))
  (bind _asbp_cable (cast `/Game/BPs/CableConnect/BP_Cable` Object)
    (:`then`
      (if (not (`self.HasCableInHand`))
        (bind _output_get (set `self.Cable` _asbp_cable))
        (`self.SetActorEnableCollision` _output_get true)
        (for _array_element (`self.K2_GetComponentsByClass` _output_get "/Script/Engine.StaticMeshComponent")
          (`PrimitiveComponent.SetSimulatePhysics` _array_element true)
          (`PrimitiveComponent.SetCollisionEnabled` _array_element "QueryAndPhysics"))
        (`PhysicsHandleComponent.GrabComponentAtLocation` (`self.PhysicsHandle`) _returnvalue "None" (`SceneComponent.K2_GetComponentLocation` _returnvalue))
        (set `self.HasCableInHand` true)
        (bind _returnvalue_2 (`KismetSystemLibrary.K2_SetTimer` null "CopyMouseLocation" 0.1 true))
        (set `self.MouseCopyTimer` _returnvalue_2)
        (return true)))
    (:`CastFailed`
      (return false))))

(fn `DetachCableAndSetTransform`
  (params (NewRotation :type "Rotator Structure") (NewLocation :type "Vector Structure") (`DetachBoth?` :type Boolean))
  (bind _returnvalue (`self.GetGrabableCablePart`))
  (bind _cable (`self.Cable`))
  (if `DetachBoth?`
    (`PhysicsHandleComponent.ReleaseComponent` (`self.PhysicsHandle`))
    (`PrimitiveComponent.SetSimulatePhysics` (`/Game/BPs/CableConnect/BP_Cable.Start` (`self.Cable`)) false)
    (`PrimitiveComponent.SetSimulatePhysics` (`/Game/BPs/CableConnect/BP_Cable.End` (`self.Cable`)) false)
    (`self.K2_SetActorLocation` _cable NewLocation false false)
    (`self.K2_SetActorRotation` _cable NewRotation false)
    (else
      (`PhysicsHandleComponent.ReleaseComponent` (`self.PhysicsHandle`))
      (`PrimitiveComponent.SetSimulatePhysics` _returnvalue false)
      (`SceneComponent.K2_SetWorldLocation` _returnvalue NewLocation false false)
      (`SceneComponent.K2_SetWorldRotation` _returnvalue NewRotation false false))))

(fn `GetGrabableCablePart`
  (returns (ReturnValue :type "StaticMeshComponent Object Reference"))
  (bind _cable (`self.Cable`))
  (return (select `bool` (`/Game/BPs/CableConnect/BP_Cable.IsCableStart?` _cable) :`false` (`/Game/BPs/CableConnect/BP_Cable.End` _cable) :`true` (`/Game/BPs/CableConnect/BP_Cable.Start` _cable))))

(fn `Interact`
  (params (`Player Character` :type "/Game/BPs/Player/BP_FirstPersonCharacter Object Reference") (PickUpItem :type "/Game/BPs/PickUps/BP_PickUpItem Object Reference"))
  (returns (UsedPickUp :type Boolean))
  (bind _cable_1 (`self.Cable_1`))
  (bind _usedpickup (`parent.Interact` `Player Character` PickUpItem))
  (if (`self.HasNewCables?`)
    (`/Engine/EditorBlueprintResources/StandardMacros.DoOnce` false
      (:`Completed`
        (`self.SetActorHiddenInGame` _cable_1 false)
        (`self.SetActorHiddenInGame` (`self.Cable_2`) false)
        (`self.SetActorHiddenInGame` (`self.Cable_4`) false)
        (`self.SetActorHiddenInGame` (`self.Cable_5`) false)
        (`self.SetActorEnableCollision` _cable_1 true)
        (`self.SetActorEnableCollision` (`self.Cable_2`) true)
        (`self.SetActorEnableCollision` (`self.Cable_4`) true)
        (`self.SetActorEnableCollision` (`self.Cable_5`) true)))
    (else
      (`/Game/BPs/BP_ItemDialogueComp.StartInteractDialogue` (`self.BP_ItemDialogueComp`))))
  (return _usedpickup))

(fn `UserConstructionScript`
  (`parent.UserConstructionScript`))