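; Possessable interactable TentGuy character who runs a dialogue and checks the player for a set of required items.
; Possession opens a dialogue widget after a short delay; ending it returns to the player, with the first return switching to the second data table and enabling item checks.
; Interact counts required items in the player's pickups and removes them once all are present.
; The dialogue condition check disables possession when three correct items are counted.
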(event `self.ReceiveBeginPlay`
  (`parent.ReceiveBeginPlay`))

(event `self.GetPossessed`
  (`parent.GetPossessed`)
  (`KismetSystemLibrary.Delay` 0.2)
  (bind _returnvalue (`|CreateWidget` "/Game/UI/Dialogue/BPW_Dialogue.BPW_Dialogue_C"))
  (bind _output_get (set `self.DialogueUIRef` _returnvalue))
  (set `/Game/UI/Dialogue/BPW_Dialogue.DialogueDataTable` (`self.StartDataTable`) _output_get)
  (set `/Game/UI/Dialogue/BPW_Dialogue.OwningObject` self _output_get)
  (`UserWidget.AddToViewport` _output_get 0)
  (add `/Game/UI/Dialogue/BPW_Dialogue.CallEnded` (`self.DialogueUIRef`) (delegate `self.ReturnToCharacter`)))

(event `self.ReturnToCharacter`
  (`parent.ReturnToCharacter`)
  (`WidgetBlueprintLibrary.SetInputMode_GameOnly` (`GameplayStatics.GetPlayerController` 0) true)
  (`Widget.RemoveFromParent` (`self.DialogueUIRef`))
  (`/Engine/EditorBlueprintResources/StandardMacros.DoOnce` false
    (:`Completed`
      (`self.ChangeDataTable`)
      (set `self.CheckArray` true))))

(event `ChangeDataTable`
  (set `self.StartDataTable` (`self.SecondDataTable`)))

(fn `GetDataTableAfterConditionCheck`
  (returns (ConditionMet :type Boolean))
  (if (== (`self.CorrectItems`) 3)
    (set `self.CanBePossessed?` false)
    (return true)
    (else
      (return false))))

(fn `Interact`
  (params (`Player Character` :type "/Game/BPs/Player/BP_FirstPersonCharacter Object Reference") (PickUpItem :type "/Game/BPs/PickUps/BP_PickUpItem Object Reference"))
  (returns (UsedPickUp :type Boolean))
  (bind _correctitems (`self.CorrectItems`))
  (`parent.Interact` `Player Character` PickUpItem)
  (`/Game/BPs/Player/BP_FirstPersonCharacter.Un/StashPickUp` `Player Character` true)
  (if (`self.CheckArray`)
    (set `self.CorrectItems` 0)
    (bind (_arrayindex _arrayelement) (`/Engine/EditorBlueprintResources/StandardMacros.ReverseForEachLoop` (`self.CorrectItemsArray`))
      (:`LoopBody`
        (if (>= (`KismetArrayLibrary.Array_Find` (`/Game/BPs/Player/BP_FirstPersonCharacter.PickUpItemArray` `Player Character`) _arrayelement) 0)
          (bind _result (`/Engine/EditorBlueprintResources/StandardMacros.IncrementInt` (`self.CorrectItems`))
            (:`  `
              (`KismetSystemLibrary.PrintString` (`KismetStringLibrary.Conv_IntToString` _result))))))
      (:`Completed`
        (`KismetSystemLibrary.PrintString` (`KismetStringLibrary.Conv_IntToString` _correctitems))
        (bind _output_get (set `self.CheckArray` (not (== _correctitems (`KismetArrayLibrary.Array_Length` (`self.CorrectItemsArray`))))))
        (if (not _output_get)
          (for _array_element (`self.CorrectItemsArray`)
            (`KismetArrayLibrary.Array_RemoveItem` (`/Game/BPs/Player/BP_FirstPersonCharacter.PickUpItemArray` (`self.Player Character`)) _array_element)))
        (return false)))
    (else
      (return false))))

(fn `UserConstructionScript`
  (`parent.UserConstructionScript`))