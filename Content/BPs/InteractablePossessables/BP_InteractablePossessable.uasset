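; Base pawn for interactable puzzles that the player possesses on interact and leaves to return to the first-person character.
; Possessing and returning blend the view target, swap Enhanced Input mapping contexts, toggle the player HUD and show or fade an optional controls prompt.
; When solved, it calls the solved-puzzle events, optionally cuts away to a camera with a smooth blend, then disables possession and returns control to the character.
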(event `self.ReceiveBeginPlay`
  (bind _asbp_first_person_character (cast `/Game/BPs/Player/BP_FirstPersonCharacter` (`GameplayStatics.GetPlayerPawn` 0)))
  (set `self.Player Character` _asbp_first_person_character))

(event `GetPossessed`
  (`EnhancedInputSubsystemInterface.RemoveMappingContext` (pcsubsystem `EnhancedInputLocalPlayerSubsystem` (`GameplayStatics.GetPlayerController` 0)) (`self.Character Mapping Context`) (struct))
  (`self.StopInput`)
  (`PlayerController.SetViewTargetWithBlend` (`GameplayStatics.GetPlayerController` 0) self (`self.SmoothPossessDuration`) (`self.Blend Func`) (`self.Blend Exp`) false)
  (`self.AddControllsToView`)
  (`KismetSystemLibrary.Delay` (`self.SmoothPossessDuration`))
  (`Controller.Possess` (`GameplayStatics.GetPlayerController` 0) self)
  (`EnhancedInputSubsystemInterface.AddMappingContext` (pcsubsystem `EnhancedInputLocalPlayerSubsystem` (`GameplayStatics.GetPlayerController` 0)) (`self.Mapping Context`) 2 (struct))
  (`Widget.SetVisibility` (`/Game/BPs/Player/BP_FirstPersonCharacter.PlayerHUD` (`self.Player Character`)) "Hidden"))

(event `ReturnToCharacter`
  (`self.SendAwayControlls`)
  (`EnhancedInputSubsystemInterface.RemoveMappingContext` (pcsubsystem `EnhancedInputLocalPlayerSubsystem` (`GameplayStatics.GetPlayerController` 0)) (`self.Mapping Context`) (struct))
  (`PlayerController.SetViewTargetWithBlend` (`GameplayStatics.GetPlayerController` 0) (`self.Player Character`) (`self.SmoothPossessDuration`) (`self.Blend Func`) (`self.Blend Exp`) false)
  (`KismetSystemLibrary.Delay` (`self.SmoothPossessDuration`))
  (`EnhancedInputSubsystemInterface.AddMappingContext` (pcsubsystem `EnhancedInputLocalPlayerSubsystem` (`GameplayStatics.GetPlayerController` 0)) (`self.Character Mapping Context`) 2 (struct))
  (`Controller.Possess` (`GameplayStatics.GetPlayerController` 0) (`self.Player Character`))
  (`EnhancedInputLibrary.FlushPlayerInput` (`GameplayStatics.GetPlayerController` 0))
  (`self.EnableInput` (`self.Player Character`) (`GameplayStatics.GetPlayerController` 0))
  (`Widget.SetVisibility` (`/Game/BPs/Player/BP_FirstPersonCharacter.PlayerHUD` (`self.Player Character`)) "Visible"))

(event `PlaySolved`
  (bind _smoothpossessduration (`self.SmoothPossessDuration`))
  (`self.SolvedPuzzleDoSMTH`)
  (`/Engine/EditorBlueprintResources/StandardMacros.IsValid` (`self.Cam`)
    (:`Is Valid`
      (`PlayerController.SetViewTargetWithBlend` (`GameplayStatics.GetPlayerController` 0) (`self.Cam`) _smoothpossessduration (`self.Blend Func`) (`self.Blend Exp`) false)
      (`KismetSystemLibrary.Delay` _smoothpossessduration)
      (`self.SolvedPuzzle`)
      (`KismetSystemLibrary.Delay` (+ _smoothpossessduration (`self.AddedWaitAfterCamChange`))))
    (:`Is Not Valid`
      _))
  (set `self.CanBePossessed?` false)
  (`self.ReturnToCharacter`))

(fn `AddControllsToView`
  (if (not (`KismetTextLibrary.TextIsEmpty` (`self.Controlls`)))
    (`/Engine/EditorBlueprintResources/StandardMacros.IsValid` (`self.PuzzleControlls`)
      (:`Is Valid`
        _)
      (:`Is Not Valid`
        (bind _returnvalue (`|CreateWidget` "/Game/UI/Puzzles/BPW_PuzzleControlls.BPW_PuzzleControlls_C" (`GameplayStatics.GetPlayerController` 0)))
        (set `self.PuzzleControlls` _returnvalue)))
    (set `/Game/UI/Puzzles/BPW_PuzzleControlls.TextPrompt` (`self.Controlls`) (`self.PuzzleControlls`))
    (`UserWidget.AddToViewport` (`self.PuzzleControlls`) 0)))

(fn `Interact`
  (params (`Player Character` :type "/Game/BPs/Player/BP_FirstPersonCharacter Object Reference") (PickUpItem :type "/Game/BPs/PickUps/BP_PickUpItem Object Reference"))
  (returns (UsedPickUp :type Boolean))
  (set `self.Player Character` `Player Character`)
  (if (`self.CanBePossessed?`)
    (`self.GetPossessed`)
    (return false)))

(fn `SendAwayControlls`
  (if (not (`KismetTextLibrary.TextIsEmpty` (`self.Controlls`)))
    (`/Game/UI/Puzzles/BPW_PuzzleControlls.FadeOutControlls` (`self.PuzzleControlls`))))

(fn `StopInput`
  (returns (`Player Character` :type "/Game/BPs/Player/BP_FirstPersonCharacter Object Reference"))
  (`self.ConsumeMovementInputVector` (`self.Player Character`))
  (`self.DisableInput` (`self.Player Character`) (`GameplayStatics.GetPlayerController` 0))
  (return (`self.Player Character`)))

(fn `UserConstructionScript`)