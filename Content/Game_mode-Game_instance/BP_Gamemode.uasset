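; Game mode that controls time of day by swapping lighting sublevels loaded as level instances.
; BeginPlay loads the starting sun level and keeps a reference to it as the current light level.
; ChangeDaytime increments a daytime index, requests unload and removal of the current instance, then loads the middle-sun or sunset level selected by index.
; A GameModeRef function returns the game mode itself.
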(event `self.ReceiveBeginPlay`
  (bind (_boutsuccess _returnvalue) (`LevelStreamingDynamic.LoadLevelInstanceBySoftObjectPtr` "/Game/Maps/Daytimes/Start_Sun.Start_Sun" (0.0 0.0 0.0) (struct) "" null))
  (set `self.CurrentLightLevel` _returnvalue))

(event `ChangeDaytime`
  (bind _result (`/Engine/EditorBlueprintResources/StandardMacros.IncrementInt` (`self.DaytimeIndex`))
    (:`  `
      (`LevelStreaming.SetIsRequestingUnloadAndRemoval` (`self.CurrentLightLevel`) true)
      (bind (_boutsuccess _returnvalue) (`LevelStreamingDynamic.LoadLevelInstanceBySoftObjectPtr` (select `int` _result :`0` "/Game/Maps/Daytimes/Middle_Sun.Middle_Sun" :`1` "/Game/Maps/Daytimes/Sunsetting.Sunsetting" :!type "World Soft Object Reference") (0.0 0.0 0.0) (struct) "" null))
      (set `self.CurrentLightLevel` _returnvalue))))

(fn `GameModeRef`
  (returns (GameMode :type "/Game/Game_mode-Game_instance/BP_Gamemode Object Reference"))
  (return self))

(fn `UserConstructionScript`)