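; BP_ScaleCube is a test actor that squashes and stretches in response to the first-person character, with a fake drop shadow.
; Two timelines lerp scale from the starting value: Squash plays on box overlap begin, Stretch on overlap end and BeginPlay, each stopping the other.
; Every tick, a downward sphere trace positions a decal, shrinking and fading it with distance through a dynamic material, hiding it without a hit.
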(event `self.ReceiveBeginPlay`
  (bind _startscale (`self.StartScale`))
  (bind _startscale_2 (`self.StartScale`))
  (set `self.StartScale` (`SceneComponent.RelativeScale3D` (`self.Scene`)))
  (`TimelineComponent.SetPlayRate` (`self.Stretch`) 1.0)
  (`TimelineComponent.SetPlayRate` (`self.Squash`) 1.0)
  (`|ExecutionSequence`
    (:`then_0`
      (bind (_direction _alpha) (`Timeline|Stretch` :!via `PlayFromStart` :!label _label)
        (:`Update`
          (`SceneComponent.SetRelativeScale3D` (`self.Scene`) (`KismetMathLibrary.VLerp` _startscale_2 (* _startscale_2 (`self.JumpStretchFactor`)) _alpha)))))
    (:`then_1`
      (bind (_direction_2 _alpha_2) (`Timeline|Squash` :!via `Stop` :!label _label_2)
        (:`Update`
          (`SceneComponent.SetRelativeScale3D` (`self.Scene`) (`KismetMathLibrary.VLerp` _startscale (* _startscale (`self.JumpSquashFactor`)) _alpha_2)))))))

(event `self.Box.OnComponentEndOverlap`
  (params (OverlappedComponent :type "PrimitiveComponent Object Reference") (OtherActor :type "Actor Object Reference") (OtherComp :type "PrimitiveComponent Object Reference") (OtherBodyIndex :type Integer))
  (cast `/Game/BPs/Player/BP_FirstPersonCharacter` OtherActor)
  (`|ExecutionSequence`
    (:`then_0`
      (goto _label :!via `PlayFromStart`))
    (:`then_1`
      (goto _label_2 :!via `Stop`))))

(event `self.Box.OnComponentBeginOverlap`
  (params (OverlappedComponent :type "PrimitiveComponent Object Reference") (OtherActor :type "Actor Object Reference") (OtherComp :type "PrimitiveComponent Object Reference") (OtherBodyIndex :type Integer) (bFromSweep :type Boolean) (SweepResult :type "HitResult Structure (by ref)"))
  (cast `/Game/BPs/Player/BP_FirstPersonCharacter` OtherActor)
  (`|ExecutionSequence`
    (:`then_0`
      (goto _label_2 :!via `PlayFromStart`))
    (:`then_1`
      (goto _label :!via `Stop`))))

(event `self.ReceiveTick`
  (params (DeltaSeconds :type "Float (single-precision)"))
  (`self.DropShadow`))

(event `DropShadow`
  (bind _returnvalue (`self.K2_GetActorLocation`))
  (bind _decal (`self.Decal`))
  (bind (_outhit _returnvalue_2) (`KismetSystemLibrary.SphereTraceSingle` _returnvalue (- _returnvalue (`KismetMathLibrary.MakeVector` 0.0 0.0 (`self.TraceDistance`))) 10.0 "TraceTypeQuery1"))
  (if _returnvalue_2
    (bind (_bblockinghit _binitialoverlap _time _distance _location) (`GameplayStatics.BreakHitResult` _outhit))
    (`SceneComponent.K2_SetWorldLocation` _decal _location false false)
    (bind _returnvalue_3 (`KismetMathLibrary.MapRangeClamped` _distance 0.0 (`self.TraceDistance`) 1.0 0.2))
    (`SceneComponent.SetRelativeScale3D` _decal (`KismetMathLibrary.Conv_DoubleToVector` _returnvalue_3))
    (`MaterialInstanceDynamic.SetScalarParameterValue` (`self.DMI_Shadow`) "Opacity" _returnvalue_3)
    (else
      (`MaterialInstanceDynamic.SetScalarParameterValue` (`self.DMI_Shadow`) "Opacity" 0.0))))

(fn `UserConstructionScript`
  (bind _returnvalue (`DecalComponent.CreateDynamicMaterialInstance` (`self.Decal`)))
  (set `self.DMI_Shadow` _returnvalue))